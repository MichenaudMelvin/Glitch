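; Blueprint helper function library that gives quick, typed access to the main player character and its controller.
; CallMainPlayer and CallBPMainPlayer cast player character 0 to MainPlayer and BP_MainPlayer respectively.
; CallBPMainPlayerController casts player controller 0 to BP_PC_MainPlayerController.
; All lookups use player index 0, so they only ever return the first player.
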(fn `CallBPMainPlayer`
  (returns (BPMainPlayer :type "/Game/Blueprint/Player/BP_MainPlayer Object Reference"))
  (return (cast `/Game/Blueprint/Player/BP_MainPlayer` (`GameplayStatics.GetPlayerCharacter` null) :!pure true)))

(fn `CallBPMainPlayerController`
  (returns (`BPPCMain Player Controller` :type "/Game/Blueprint/Player/Controllers/BP_PC_MainPlayerController Object Reference"))
  (return (cast `/Game/Blueprint/Player/Controllers/BP_PC_MainPlayerController` (`GameplayStatics.GetPlayerController` null) :!pure true)))

(fn `CallMainPlayer`
  (returns (MainPlayer :type "MainPlayer Object Reference"))
  (return (cast `MainPlayer` (`GameplayStatics.GetPlayerCharacter` null) :!pure true)))