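; Blueprint function library of small helpers for class checks and Blackboard access.
; CheckTargetClass tests an exact class match and CheckParentClass tests inheritance, both passing the object and class back alongside the result.
; Typed Set and Get wrappers cover Blackboard values from bool and enum to object, rotator and string, turning the supplied key into a literal Name before each call.
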(fn `CheckParentClass`
  (params (TargetObject :type "Object Object Reference") (ParentClass :type "Object Class Reference"))
  (returns (ReturnValue :type Boolean) (ReturnObject :type "Object Object Reference") (ReturnClass :type "Object Class Reference"))
  (return (`KismetMathLibrary.ClassIsChildOf` (`GameplayStatics.GetObjectClass` TargetObject) (`local.ParentClass`)) (`local.TargetObject`) (`local.ParentClass`)))

(fn `CheckTargetClass`
  (params (TargetObject :type "Object Object Reference") (TargetClass :type "Object Class Reference"))
  (returns (ReturnValue :type Boolean) (ReturnObject :type "Object Object Reference") (ReturnClass :type "Object Class Reference"))
  (return (== (`GameplayStatics.GetObjectClass` TargetObject) (`local.TargetClass`)) (`local.TargetObject`) (`local.TargetClass`)))

(fn `GetBlackboardValueAsBool`
  (params (BlackBoard :type "BlackboardComponent Object Reference") (Value :type Name))
  (returns (ReturnValue :type Boolean))
  (return (`BlackboardComponent.GetValueAsBool` BlackBoard (`KismetSystemLibrary.MakeLiteralName` Value))))

(fn `GetBlackboardValueAsClass`
  (params (BlackBoard :type "BlackboardComponent Object Reference") (Value :type Name))
  (returns (ReturnValue :type "Object Class Reference"))
  (return (`BlackboardComponent.GetValueAsClass` BlackBoard (`KismetSystemLibrary.MakeLiteralName` Value))))

(fn `GetBlackboardValueAsEnum`
  (params (BlackBoard :type "BlackboardComponent Object Reference") (Value :type Name))
  (returns (ReturnValue :type Byte))
  (return (`BlackboardComponent.GetValueAsEnum` BlackBoard (`KismetSystemLibrary.MakeLiteralName` Value))))

(fn `GetBlackboardValueAsFloat`
  (params (BlackBoard :type "BlackboardComponent Object Reference") (Value :type Name))
  (returns (ReturnValue :type "Float (double-precision)"))
  (return (`BlackboardComponent.GetValueAsFloat` BlackBoard (`KismetSystemLibrary.MakeLiteralName` Value))))

(fn `GetBlackboardValueAsInt`
  (params (BlackBoard :type "BlackboardComponent Object Reference") (Value :type Name))
  (returns (ReturnValue :type Integer))
  (return (`BlackboardComponent.GetValueAsInt` BlackBoard (`KismetSystemLibrary.MakeLiteralName` Value))))

(fn `GetBlackboardValueAsName`
  (params (BlackBoard :type "BlackboardComponent Object Reference") (Value :type Name))
  (returns (ReturnValue :type Name))
  (return (`BlackboardComponent.GetValueAsName` BlackBoard (`KismetSystemLibrary.MakeLiteralName` Value))))

(fn `GetBlackboardValueAsObject`
  (params (BlackBoard :type "BlackboardComponent Object Reference") (Value :type Name))
  (returns (ReturnValue :type "Object Object Reference"))
  (return (`BlackboardComponent.GetValueAsObject` BlackBoard (`KismetSystemLibrary.MakeLiteralName` Value))))

(fn `GetBlackboardValueAsRotator`
  (params (BlackBoard :type "BlackboardComponent Object Reference") (Value :type Name))
  (returns (ReturnValue :type "Rotator Structure"))
  (return (`BlackboardComponent.GetValueAsRotator` BlackBoard (`KismetSystemLibrary.MakeLiteralName` Value))))

(fn `GetBlackboardValueAsString`
  (params (BlackBoard :type "BlackboardComponent Object Reference") (Value :type Name))
  (returns (ReturnValue :type String))
  (return (`BlackboardComponent.GetValueAsString` BlackBoard (`KismetSystemLibrary.MakeLiteralName` Value))))

(fn `GetBlackboardValueAsVector`
  (params (BlackBoard :type "BlackboardComponent Object Reference") (Value :type Name))
  (returns (ReturnValue :type "Vector Structure"))
  (return (`BlackboardComponent.GetValueAsVector` BlackBoard (`KismetSystemLibrary.MakeLiteralName` Value))))

(fn `SetBlackboardValueAsBool`
  (params (BlackBoard :type "BlackboardComponent Object Reference") (Value :type Name) (BoolValue :type Boolean))
  (`BlackboardComponent.SetValueAsBool` BlackBoard (`KismetSystemLibrary.MakeLiteralName` Value) (`local.BoolValue`))
  (return))

(fn `SetBlackboardValueAsClass`
  (params (BlackBoard :type "BlackboardComponent Object Reference") (Value :type Name) (ClassValue :type "Object Class Reference"))
  (`BlackboardComponent.SetValueAsClass` BlackBoard (`KismetSystemLibrary.MakeLiteralName` Value) (`local.ClassValue`))
  (return))

(fn `SetBlackboardValueAsEnum`
  (params (BlackBoard :type "BlackboardComponent Object Reference") (Value :type Name) (EnumValue :type Byte))
  (`BlackboardComponent.SetValueAsEnum` BlackBoard (`KismetSystemLibrary.MakeLiteralName` Value) (`local.EnumValue`))
  (return))

(fn `SetBlackboardValueAsFloat`
  (params (BlackBoard :type "BlackboardComponent Object Reference") (Value :type Name) (FloatValue :type "Float (double-precision)"))
  (`BlackboardComponent.SetValueAsFloat` BlackBoard (`KismetSystemLibrary.MakeLiteralName` Value) (`local.FloatValue`))
  (return))

(fn `SetBlackboardValueAsInt`
  (params (BlackBoard :type "BlackboardComponent Object Reference") (Value :type Name) (IntValue :type Integer))
  (`BlackboardComponent.SetValueAsInt` BlackBoard (`KismetSystemLibrary.MakeLiteralName` Value) (`local.IntValue`))
  (return))

(fn `SetBlackboardValueAsName`
  (params (BlackBoard :type "BlackboardComponent Object Reference") (Value :type Name) (NameValue :type Name))
  (`BlackboardComponent.SetValueAsName` BlackBoard (`KismetSystemLibrary.MakeLiteralName` Value) (`local.NameValue`))
  (return))

(fn `SetBlackboardValueAsObject`
  (params (BlackBoard :type "BlackboardComponent Object Reference") (Value :type Name) (ObjectValue :type "Object Object Reference"))
  (`BlackboardComponent.SetValueAsObject` BlackBoard (`KismetSystemLibrary.MakeLiteralName` Value) (`local.ObjectValue`))
  (return))

(fn `SetBlackboardValueAsRotator`
  (params (BlackBoard :type "BlackboardComponent Object Reference") (Value :type Name) (RotatorValue :type "Rotator Structure"))
  (`BlackboardComponent.SetValueAsRotator` BlackBoard (`KismetSystemLibrary.MakeLiteralName` Value) (`local.RotatorValue`))
  (return))

(fn `SetBlackboardValueAsString`
  (params (BlackBoard :type "BlackboardComponent Object Reference") (Value :type Name) (StringValue :type String))
  (`BlackboardComponent.SetValueAsString` BlackBoard (`KismetSystemLibrary.MakeLiteralName` Value) (`local.StringValue`))
  (return))

(fn `SetBlackboardValueAsVector`
  (params (BlackBoard :type "BlackboardComponent Object Reference") (Value :type Name) (VectorValue :type "Vector Structure"))
  (`BlackboardComponent.SetValueAsVector` BlackBoard (`KismetSystemLibrary.MakeLiteralName` Value) (`local.VectorValue`))
  (return))