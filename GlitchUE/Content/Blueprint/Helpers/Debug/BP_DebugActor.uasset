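; BP_DebugActor is a debug helper that shows the name of the object the main player's interaction trace is hitting.
; On BeginPlay it creates a WBP_DebugWidget, caches the player and controller, enables input, and destroys itself if no valid player exists.
; The P key toggles the widget in the viewport.
; Each Tick reruns the player's InteractionLineTrace and, on a hit, rebuilds the widget's text list.
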(event `self.ReceiveBeginPlay`
  (bind _returnvalue (`|CreateWidget` "/Game/Blueprint/Helpers/Debug/WBP_DebugWidget.WBP_DebugWidget_C"))
  (set `self.DebugWidget` _returnvalue)
  (set `self.MainPlayer` (cast `MainPlayer` (`GameplayStatics.GetPlayerCharacter` 0) :!pure true))
  (bind _output_get (set `self.MainPlayerController` (cast `/Game/Blueprint/Player/Controllers/BP_PC_MainPlayerController` (`GameplayStatics.GetPlayerController` 0) :!pure true)))
  (`self.EnableInput` _output_get)
  (`/Engine/EditorBlueprintResources/StandardMacros.IsValid` (`self.MainPlayer`)
    (:`Is Not Valid`
      (`self.K2_DestroyActor`))))

(event `Key|P`
  (params (Key :type "Key Structure"))
  (:`Pressed`
    (`/Engine/EditorBlueprintResources/StandardMacros.FlipFlop`
      (:`A`
        (`UserWidget.AddToViewport` (`self.DebugWidget`) 0))
      (:`B`
        (`Widget.RemoveFromParent` (`self.DebugWidget`))))))

(event `self.ReceiveTick`
  (params (DeltaSeconds :type "Float (single-precision)"))
  (bind (_returnvalue _outhit) (`/Game/Blueprint/Player/BP_MainPlayer.InteractionLineTrace` (cast `/Game/Blueprint/Player/BP_MainPlayer` (`self.MainPlayer`) :!pure true)))
  (if _returnvalue
    (`KismetArrayLibrary.Array_Clear` (`self.TextList`))
    (`KismetArrayLibrary.Array_Add` (`self.TextList`) (`KismetStringLibrary.Concat_StrStr` "Target object : " (`KismetSystemLibrary.GetObjectName` (`.HitActor` (`GameplayStatics.BreakHitResult` _outhit)))))
    (`/Game/Blueprint/Helpers/Debug/WBP_DebugWidget.UpdateText` (`self.DebugWidget`) (`self.TextList`))))

(fn `UserConstructionScript`)