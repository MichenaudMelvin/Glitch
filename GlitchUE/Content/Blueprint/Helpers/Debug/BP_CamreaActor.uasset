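; BP_CamreaActor is a debug helper camera that can temporarily take over the player's view.
; Posses blends the view target to this actor, and Unposses blends it back to the player character and clears the tracking timer.
; FaceToPlayer rotates the camera toward the character, either once on possess or, with AlwaysFaceToPlayer, through a very short looping timer instead of Tick.
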(event `Posses`
  (`PlayerController.SetViewTargetWithBlend` (`GameplayStatics.GetPlayerController` 0) self 1.0 "VTBlend_Linear" 0.0 false)
  (if (`self.AlwaysFaceToPlayer`)
    (bind _returnvalue (`KismetSystemLibrary.K2_SetTimerDelegate` (`|CreateDelegate` :!event `FaceToPlayer`) 0.0001 true))
    (set `self.FaceToPlayerTimer` _returnvalue)
    (else
      (`self.FaceToPlayer`))))

(event `Unposses`
  (`PlayerController.SetViewTargetWithBlend` (`GameplayStatics.GetPlayerController` 0) (`GameplayStatics.GetPlayerCharacter` 0) 1.0 "VTBlend_Linear" 0.0 false)
  (`KismetSystemLibrary.K2_ClearAndInvalidateTimerHandle` (`self.FaceToPlayerTimer`)))

(event `FaceToPlayer`
  (`SceneComponent.K2_SetWorldRotation` (`self.Camera`) (`KismetMathLibrary.FindLookAtRotation` (`self.K2_GetActorLocation`) (`self.K2_GetActorLocation` (`GameplayStatics.GetPlayerCharacter` 0))) false false))

(fn `UserConstructionScript`)