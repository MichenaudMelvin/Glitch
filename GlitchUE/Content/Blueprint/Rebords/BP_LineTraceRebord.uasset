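; Ledge (rebord) detector that flags when the main player is beneath it, exposing the result as CanInteract.
; Every tick it line-traces straight down from StartTrace over TraceLength on the Visibility channel, drawing debug for one frame, and checks whether the hit actor is BP_MainPlayer.
; Two DoOnce nodes reset each other, so CanInteract is written only when detection starts or stops.
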(event `self.ReceiveTick`
  (params (DeltaSeconds :type "Float (single-precision)"))
  (bind _returnvalue (`SceneComponent.K2_GetComponentLocation` (`self.StartTrace`)))
  (bind (_outhit _returnvalue_2) (`KismetSystemLibrary.LineTraceSingle` :`Start` _returnvalue :`End` (`KismetMathLibrary.MakeVector` (.x _returnvalue) (.y _returnvalue) (- (.z _returnvalue) (`self.TraceLength`))) :`TraceChannel` "TraceTypeQuery1" :`bTraceComplex` true :`DrawDebugType` "ForOneFrame"))
  (if _returnvalue_2
    (if (`/Game/Blueprint/Helpers/FunctionLibrary/BP_UsefullFunctions.CheckTargetClass` (`.HitActor` (`GameplayStatics.BreakHitResult` _outhit)) "/Game/Blueprint/Player/BP_MainPlayer.BP_MainPlayer_C")
      (`/Engine/EditorBlueprintResources/StandardMacros.DoOnce` false :!label _label
        (:`Completed`
          (set `self.CanInteract` true)
          (goto _label_2 :!via `Reset`)))
      (else
        _)))
  (`/Engine/EditorBlueprintResources/StandardMacros.DoOnce` false :!label _label_2
    (:`Completed`
      (set `self.CanInteract` false)
      (goto _label :!via `Reset`))))

(fn `UserConstructionScript`
  (`parent.UserConstructionScript`))