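; BP_MainRebord is a climbable ledge ("rebord") that moves the player onto it when interacted with.
; On BeginPlay it labels itself with its object name and registers its Rebord mesh with the interactable component.
; An interaction, gated by CanInteract, calls Climb, which moves the player's capsule through two marker points, Location1 then Location, using MoveComponentTo.
; A timeline-driven lerp movement remains in the graph but never runs.
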(event `self.ReceiveBeginPlay`
  (`TextRenderComponent.K2_SetText` (`self.Name`) (`KismetTextLibrary.Conv_StringToText` (`KismetSystemLibrary.GetObjectName` self)))
  (`BlueprintSetLibrary.Set_Add` (`/Game/Blueprint/Interactables/AC_Interactable.InteractableStaticMeshes` (`self.AC_Interactable`)) (`self.Rebord`)))

(event `Climb`
  (params (MainPlayer :type "/Game/Blueprint/Player/BP_MainPlayer Object Reference"))
  (`KismetSystemLibrary.MoveComponentTo` (`Character.CapsuleComponent` MainPlayer) (`SceneComponent.K2_GetComponentLocation` (`self.Location1`)))
  (`KismetSystemLibrary.MoveComponentTo` (`Character.CapsuleComponent` MainPlayer) (`SceneComponent.K2_GetComponentLocation` (`self.Location`))))

(event `self.AC_Interactable.OnInteract`
  (params (BPMainPlayerController :type "/Game/Blueprint/Player/Controllers/BP_PC_MainPlayerController Object Reference") (BPMainPlayer :type "/Game/Blueprint/Player/BP_MainPlayer Object Reference"))
  (if (`self.CanInteract`)
    (`self.Climb` BPMainPlayer)))

(fn `UserConstructionScript`)