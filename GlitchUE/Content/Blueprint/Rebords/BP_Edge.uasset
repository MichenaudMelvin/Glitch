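; Ledge actor that lets BP_MainPlayer cling to an edge, built from two box triggers sized by BoxLength.
; UpperEdge overlap rebinds player interaction, while MovePlayerToEdge turns and moves the capsule down to the LowerEdge cling point with collision ignored.
; That point is projected along the edge via Pythagoras, its side chosen by actor yaw.
; LowerEdge overlap attaches the player, zeroing gravity and switching to cling controls; leaving detaches.
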(event `self.ReceiveBeginPlay`
  (bind _bpmainplayer (`/Game/Blueprint/Helpers/FunctionLibrary/BP_CallElements.CallBPMainPlayer`))
  (`KismetSystemLibrary.Delay` 0.2)
  (`/Engine/EditorBlueprintResources/StandardMacros.IsValid` _bpmainplayer ; For simulation mode
    (:`Is Valid`
      (bind _output_get (set `self.Player` _bpmainplayer))
      (set `self.PlayerController` (`/Game/Blueprint/Player/BP_MainPlayer.MainPlayerController` _output_get)))))

(event `self.UpperEdge.OnComponentBeginOverlap`
  (params (OverlappedComponent :type "PrimitiveComponent Object Reference") (OtherActor :type "Actor Object Reference") (OtherComp :type "PrimitiveComponent Object Reference") (OtherBodyIndex :type Integer) (bFromSweep :type Boolean) (SweepResult :type "HitResult Structure (by ref)"))
  ;[1 1 1] UpperEdge
  (if (`/Game/Blueprint/Helpers/FunctionLibrary/BP_UsefullFunctions.CheckTargetClass` OtherActor "/Game/Blueprint/Player/BP_MainPlayer.BP_MainPlayer_C")
    (`/Engine/EditorBlueprintResources/StandardMacros.IsValid` (`/Game/Blueprint/Player/BP_MainPlayer.CurrentCheckedObject` (`self.Player`))
      (:`Is Not Valid`
        (set `/Game/Blueprint/Player/BP_MainPlayer.CurrentEdge` self (`self.Player`))
        (`self.RebindPlayerInteraction`)))))

(event `MovePlayerToEdge`
  (bind _capsulecomponent (`Character.CapsuleComponent` (`self.Player`)))
  (`PrimitiveComponent.SetCollisionResponseToAllChannels` (`Character.CapsuleComponent` (`self.Player`)) "ECR_Ignore")
  (`MainPlayer.LookAtTarget` (`self.Player`) (`UsefullFunctions.AddToRotator` (`SceneComponent.K2_GetComponentRotation` (`self.LowerEdge`)) 0.0 0.0 90.0) (`|CreateDelegate` :!event `End`) 0.5)
  (bind _output_get (set `self.TargetVector` (`self.GetLowerEdgeClingLocation`)))
  (`KismetSystemLibrary.MoveComponentTo` (`Character.CapsuleComponent` (`self.Player`)) (`KismetMathLibrary.MakeVector` (.x _output_get) (.y _output_get) (.z (`self.K2_GetActorLocation` (`self.Player`)))) (`self.GetLowerEgdeRotator`) false false 0.25)
  (`KismetSystemLibrary.MoveComponentTo` (`Character.CapsuleComponent` (`self.Player`)) (`self.TargetVector`) (`SceneComponent.RelativeRotation` (`Character.CapsuleComponent` (`self.Player`))) false false 0.25)
  (`self.AttachPlayerToEdge`)
  (`PrimitiveComponent.SetCollisionResponseToAllChannels` _capsulecomponent "ECR_Block")
  (`PrimitiveComponent.SetCollisionResponseToChannel` _capsulecomponent "ECC_Visibility" "ECR_Ignore"))

(event `self.UpperEdge.OnComponentEndOverlap`
  (params (OverlappedComponent :type "PrimitiveComponent Object Reference") (OtherActor :type "Actor Object Reference") (OtherComp :type "PrimitiveComponent Object Reference") (OtherBodyIndex :type Integer))
  ;[1 1 1] UpperEdge
  (if (`/Game/Blueprint/Helpers/FunctionLibrary/BP_UsefullFunctions.CheckTargetClass` OtherActor "/Game/Blueprint/Player/BP_MainPlayer.BP_MainPlayer_C")
    (`/Engine/EditorBlueprintResources/StandardMacros.IsValid` (`/Game/Blueprint/Player/BP_MainPlayer.CurrentCheckedObject` (`self.Player`))
      (:`Is Not Valid`
        (set `/Game/Blueprint/Player/BP_MainPlayer.CurrentEdge` null (`self.Player`))
        (`/Game/Blueprint/Player/Controllers/BP_PC_MainPlayerController.BindInteraction` (`self.PlayerController`))))))

(event `self.LowerEdge.OnComponentBeginOverlap`
  (params (OverlappedComponent :type "PrimitiveComponent Object Reference") (OtherActor :type "Actor Object Reference") (OtherComp :type "PrimitiveComponent Object Reference") (OtherBodyIndex :type Integer) (bFromSweep :type Boolean) (SweepResult :type "HitResult Structure (by ref)"))
  ;[1 1 1] LowerEdge
  (if (`/Game/Blueprint/Helpers/FunctionLibrary/BP_UsefullFunctions.CheckTargetClass` OtherActor "/Game/Blueprint/Player/BP_MainPlayer.BP_MainPlayer_C")
    (`self.AttachPlayerToEdge`)))

(event `self.LowerEdge.OnComponentEndOverlap`
  (params (OverlappedComponent :type "PrimitiveComponent Object Reference") (OtherActor :type "Actor Object Reference") (OtherComp :type "PrimitiveComponent Object Reference") (OtherBodyIndex :type Integer))
  ;[1 1 1] LowerEdge
  (if (`/Game/Blueprint/Helpers/FunctionLibrary/BP_UsefullFunctions.CheckTargetClass` OtherActor "/Game/Blueprint/Player/BP_MainPlayer.BP_MainPlayer_C")
    (`/Game/Blueprint/Player/BP_MainPlayer.DetachFromEdge` (`self.Player`))))

(event `End`)

(fn `AttachPlayerToEdge`
  (bind _playercontroller (`self.PlayerController`))
  (bind _player (`self.Player`))
  (bind _charactermovement (`Character.CharacterMovement` _player))
  (set `/Game/Blueprint/Player/BP_MainPlayer.CurrentEdge` self _player)
  (set `CharacterMovementComponent.GravityScale` 0.0 _charactermovement)
  (set `MovementComponent.Velocity` (0.0 0.0 0.0) _charactermovement)
  (`Character.StopJumping` _player)
  (`SceneComponent.K2_SetWorldRotation` (`Character.CapsuleComponent` _player) (`self.GetLowerEgdeRotator`) false false)
  (`self.K2_SetActorLocation` (`self.Player`) (`self.GetEdgeToClingLocation`) false false)
  (`MainPlayerController.UnbindGlitch` _playercontroller)
  (`MainPlayerController.UnbindConstruction` _playercontroller)
  (`MainPlayerController.UnbindOpenSelectionWheel` _playercontroller)
  (`MainPlayerController.UnbindMouseScroll` _playercontroller)
  (`MainPlayerController.BindClingMovement` _playercontroller)
  (return))

(fn `GetDistanceBetweenTheEdges`
  (returns (Distance :type "Float (double-precision)"))
  (return (`KismetMathLibrary.Vector_Distance` (`KismetMathLibrary.MakeVector` (.x (`SceneComponent.K2_GetComponentLocation` (`self.UpperEdge`))) (.y (`SceneComponent.K2_GetComponentLocation` (`self.UpperEdge`)))) (`KismetMathLibrary.MakeVector` (.x (`SceneComponent.K2_GetComponentLocation` (`self.LowerEdge`))) (.y (`SceneComponent.K2_GetComponentLocation` (`self.LowerEdge`)))))))

(fn `GetEdgeToClingLocation`
  (returns (ReturnValue :type "Vector Structure"))
  (return (`KismetMathLibrary.MakeVector` (.x (`self.K2_GetActorLocation` (`self.Player`))) (.y (`self.K2_GetActorLocation` (`self.Player`))) (.z (`SceneComponent.K2_GetComponentLocation` (`self.LowerEdge`))))))

(fn `GetLowerEdgeClingLocation`
  (returns (Result :type "Vector Structure"))
  (bind _returnvalue (* (`self.GetActorForwardVector`) (`KismetMathLibrary.Sqrt` (- (`KismetMathLibrary.Square` (`KismetMathLibrary.Vector_Distance` (`KismetMathLibrary.MakeVector` (.x (`SceneComponent.K2_GetComponentLocation` (`self.LowerEdge`))) (.y (`SceneComponent.K2_GetComponentLocation` (`self.LowerEdge`)))) (`KismetMathLibrary.MakeVector` (.x (`self.K2_GetActorLocation` (`self.Player`))) (.y (`self.K2_GetActorLocation` (`self.Player`)))))) (`KismetMathLibrary.Square` (`self.GetDistanceBetweenTheEdges`))))))
  (return (+ (`SceneComponent.K2_GetComponentLocation` (`self.LowerEdge`)) (`KismetMathLibrary.SelectVector` _returnvalue (* _returnvalue -1.0) (`self.SelectEdgeBool`)))))

(fn `GetLowerEgdeRotator`
  (returns (Result :type "Rotator Structure"))
  (return (`UsefullFunctions.AddToRotator` (`SceneComponent.K2_GetComponentRotation` (`self.LowerEdge`)) 0.0 0.0 90.0)))

(fn `RebindPlayerInteraction`
  (bind _playercontroller (`self.PlayerController`))
  (clear `MainPlayerController.OnInteractPlayer` _playercontroller)
  (add `MainPlayerController.OnInteractPlayer` _playercontroller (`|CreateDelegate` :!event `MovePlayerToEdge`))
  (return))

(fn `SelectEdgeBool`
  (returns (Value :type Boolean))
  (bind _yaw (.yaw (`self.K2_GetActorRotation`)))
  (if (> _yaw 90.0)
    (return (> (.x (`self.K2_GetActorLocation`)) (.x (`self.K2_GetActorLocation` (`self.Player`)))))
    (elif (< _yaw -90.0)
      (return (> (.y (`self.K2_GetActorLocation`)) (.y (`self.K2_GetActorLocation` (`self.Player`)))))
      (else
        (return (< (.x (`self.K2_GetActorLocation`)) (.x (`self.K2_GetActorLocation` (`self.Player`)))))))))

(fn `UpdateBoxExtent`
  (params (Box :type "BoxComponent Object Reference"))
  (`BoxComponent.SetBoxExtent` Box (`KismetMathLibrary.MakeVector` (`self.BoxLength`) 5.0 3.0) false)
  (return))

(fn `UserConstructionScript`
  (`self.UpdateBoxExtent` (`self.UpperEdge`))
  (`self.UpdateBoxExtent` (`self.LowerEdge`)))