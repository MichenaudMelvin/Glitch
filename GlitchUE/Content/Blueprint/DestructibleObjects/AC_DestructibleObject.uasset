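; AC_DestructibleObject is an actor component that gives its owner health and optional destruction.
; Health starts at the maximum, and TakeDamages subtracts from it with clamping, then signals that damage was received.
; At zero health it signals depletion and destroys the owning actor if configured.
; An optional looping timer serves as a health debug display, with PrintHealth printing the current value on screen.
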(event `self.ReceiveBeginPlay`
  (set `self.CurrentHealth` (`self.MaxHealth`))
  (if (`self.ShowHealth`)
    (`KismetSystemLibrary.K2_SetTimerDelegate` (`|CreateDelegate` :!event `PrintHealth`) 0.1 true)))

(fn `PrintHealth`
  (`/Game/Blueprint/Helpers/FunctionLibrary/BP_UsefullFunctions.Print` (`KismetStringLibrary.Conv_DoubleToString` (`self.CurrentHealth`)) true false (struct :`R` 0.95784 :`B` 1.0 :`A` 1.0) 0.1)
  (return))

(fn `TakeDamages`
  (params (Damages :type "Float (double-precision)"))
  (bind _output_get (set `self.CurrentHealth` (`KismetMathLibrary.FClamp` (- (`self.CurrentHealth`) Damages) 0.0 (`self.MaxHealth`))))
  (`self.OnReciveDamages`)
  (if (== _output_get 0.0)
    (`self.OnHealthNull`)
    (if (`self.DoDestroyWhenNoHealth`)
      (`Actor.K2_DestroyActor` (`self.GetOwner`))
      (return)
      (else
        (return)))
    (else
      (return))))