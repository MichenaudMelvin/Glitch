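; BP_CameraController is an AI controller for a camera that detects the player by sight.
; On each perception update it filters for sight stimuli and checks whether the sensed actor is BP_MainPlayer.
; On a match it writes the player and their current location to the Blackboard, without checking whether sight was gained or lost.
; BeginPlay and construction defer to the parent class.
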(event `self.ReceiveBeginPlay`
  (`parent.ReceiveBeginPlay`))

(event `self.PerceptionUpdate`
  (params (Actor :type "Actor Object Reference") (Stimulus :type "AIStimulus Structure"))
  (bind (_returnvalue _returnobject) (`/Game/Blueprint/Helpers/FunctionLibrary/BP_UsefullFunctions.CheckTargetClass` Actor "/Game/Blueprint/Player/BP_MainPlayer.BP_MainPlayer_C"))
  (bind _asbp_main_player (cast `/Game/Blueprint/Player/BP_MainPlayer` _returnobject :!pure true))
  (`parent.PerceptionUpdate` Actor Stimulus)
  (bind _returnvalue_2 (`AIPerceptionSystem.GetSenseClassForStimulus` Stimulus))
  (if (== _returnvalue_2 "/Script/AIModule.AISense_Sight")
    (if _returnvalue
      (`/Game/Blueprint/Helpers/FunctionLibrary/BP_UsefullFunctions.SetBlackboardValueAsObject` (`self.Blackboard`) "Player" _asbp_main_player)
      (`/Game/Blueprint/Helpers/FunctionLibrary/BP_UsefullFunctions.SetBlackboardValueAsVector` (`self.Blackboard`) "PlayerLocation" (`self.K2_GetActorLocation` _asbp_main_player)))))

(fn `UserConstructionScript`
  (`parent.UserConstructionScript`))