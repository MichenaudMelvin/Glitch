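; AI security camera pawn whose behavior and rotation are configured through its AI controller's blackboard.
; On BeginPlay it seeds the blackboard with its origin location, behavior enum, fixed rotation limits and rotation speed; the movement logic itself lives outside this graph.
; Its Sight component's see and lose-player events both pass the investigate-time percentage to a temporary sight indication widget.
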(event `self.ReceiveBeginPlay`
  (`parent.ReceiveBeginPlay`)
  (bind _output_get (set `self.AIController` (cast `/Game/Blueprint/AI/BP_MainAIController` (`self.GetController`) :!pure true)))
  (bind _output_get_2 (set `self.Blackboard` (`AIBlueprintHelperLibrary.GetBlackboard` _output_get)))
  (`/Game/Blueprint/Helpers/FunctionLibrary/BP_UsefullFunctions.SetBlackboardValueAsVector` _output_get_2 "OriginalPosition" (`self.K2_GetActorLocation`))
  (`/Game/Blueprint/Helpers/FunctionLibrary/BP_UsefullFunctions.SetBlackboardValueAsEnum` (`self.Blackboard`) "CameraBehavior" (`self.Behavior`))
  (`/Game/Blueprint/Helpers/FunctionLibrary/BP_UsefullFunctions.SetBlackboardValueAsFloat` (`self.Blackboard`) "MaxRotation" 90.0)
  (`/Game/Blueprint/Helpers/FunctionLibrary/BP_UsefullFunctions.SetBlackboardValueAsFloat` (`self.Blackboard`) "MinRotation" -90.0)
  (`/Game/Blueprint/Helpers/FunctionLibrary/BP_UsefullFunctions.SetBlackboardValueAsFloat` (`self.Blackboard`) "SpeedRotation" (`self.SpeedRotation`)))

(event `self.Sight.OnSightPlayer`
  (params (InvestigateTimePercent :type "Float (single-precision)"))
  (`/Game/Blueprint/AI/Temp/WBP_SightIndication.TEMP_Time` (cast `/Game/Blueprint/AI/Temp/WBP_SightIndication` (`WidgetComponent.GetWidget` (`self.TEMP_SightWidget`)) :!pure true) InvestigateTimePercent))

(event `self.Sight.OnLooseSightPlayer`
  (params (InvestigateTimePercent :type "Float (single-precision)"))
  (`/Game/Blueprint/AI/Temp/WBP_SightIndication.TEMP_Time` (cast `/Game/Blueprint/AI/Temp/WBP_SightIndication` (`WidgetComponent.GetWidget` (`self.TEMP_SightWidget`)) :!pure true) InvestigateTimePercent))

(fn `UserConstructionScript`)