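; AI controller for the Focus Catalyseur AI, which tracks perceived BP_Catalyseur actors through its blackboard.
; On BeginPlay it caches all catalyseurs in CatalyseurList and writes the first BP_Nexus location to NexusLocation.
; Perception updates extend the parent handler, storing any catalyseur as CurrentFocusedCatalyseur without checking whether it was sensed or lost.
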(event `self.ReceiveBeginPlay`
  (`parent.ReceiveBeginPlay`)
  (bind _outactors (`GameplayStatics.GetAllActorsOfClass` "/Game/Blueprint/Nexus/BP_Catalyseur.BP_Catalyseur_C"))
  (set `self.CatalyseurList` _outactors)
  (bind _outactors_2 (`GameplayStatics.GetAllActorsOfClass` "/Game/Blueprint/Nexus/BP_Nexus.BP_Nexus_C"))
  (`/Game/Blueprint/Helpers/FunctionLibrary/BP_UsefullFunctions.SetBlackboardValueAsVector` (`self.Blackboard`) "NexusLocation" (`self.K2_GetActorLocation` (`|GetArrayItem` _outactors_2))))

(event `self.PerceptionUpdate`
  (params (Actor :type "Actor Object Reference") (Stimulus :type "AIStimulus Structure"))
  (bind (_returnvalue _returnobject) (`/Game/Blueprint/Helpers/FunctionLibrary/BP_UsefullFunctions.CheckTargetClass` Actor "/Game/Blueprint/Nexus/BP_Catalyseur.BP_Catalyseur_C"))
  (`parent.PerceptionUpdate` Actor Stimulus)
  (if _returnvalue
    (`/Game/Blueprint/Helpers/FunctionLibrary/BP_UsefullFunctions.SetBlackboardValueAsObject` (`self.Blackboard`) "CurrentFocusedCatalyseur" _returnobject)))

(fn `UserConstructionScript`
  (`parent.UserConstructionScript`))