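; BP_FocusAIController is a child AI controller that seeds the blackboard for the FocusAI enemy type.
; On BeginPlay, after the parent logic, it writes its AttackDistance and the first BP_Nexus actor found in the level to the AttackDistance and Nexus keys.
; Perception updates and construction pass straight through to the parent class.
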(event `self.ReceiveBeginPlay`
  (`parent.ReceiveBeginPlay`)
  (`/Game/Blueprint/Helpers/FunctionLibrary/BP_UsefullFunctions.SetBlackboardValueAsFloat` (`self.Blackboard`) "AttackDistance" (`self.AttackDistance`))
  (bind _outactors (`GameplayStatics.GetAllActorsOfClass` "/Game/Blueprint/Nexus/BP_Nexus.BP_Nexus_C"))
  (`/Game/Blueprint/Helpers/FunctionLibrary/BP_UsefullFunctions.SetBlackboardValueAsObject` (`self.Blackboard`) "Nexus" (`|GetArrayItem` _outactors)))

(event `self.PerceptionUpdate`
  (params (Actor :type "Actor Object Reference") (Stimulus :type "AIStimulus Structure"))
  (`parent.PerceptionUpdate` Actor Stimulus))

(fn `UserConstructionScript`
  (`parent.UserConstructionScript`))