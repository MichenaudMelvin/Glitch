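; BP_MainAIController is an AI controller that runs a behavior tree and feeds it perception data about the player.
; On BeginPlay it starts the tree and writes StunTime to the blackboard.
; Perception updates are filtered to the sight sense, storing the latest stimulus and actor.
; If the sighted actor passes a BP_MainPlayer class check, its reference and location go to the blackboard, without checking whether it was successfully sensed.
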(event `self.ReceiveBeginPlay`
  (`self.RunBehaviorTree` (`self.BehaviorTree`))
  (`/Game/Blueprint/Helpers/FunctionLibrary/BP_UsefullFunctions.SetBlackboardValueAsFloat` (`self.Blackboard`) "StunTime" (`self.StunTime`)))

(event `self.AIPerception.OnTargetPerceptionUpdated`
  (params (Actor :type "Actor Object Reference") (Stimulus :type "AIStimulus Structure"))
  (`self.TargetPerceptionUpdatedEvent` Actor Stimulus))

(event `TargetPerceptionUpdatedEvent`
  (params (Actor :type "Actor Object Reference") (Stimulus :type "AIStimulus Structure"))
  (bind _currentsightactor (`self.CurrentSightActor`))
  (bind (_returnvalue _returnobject) (`/Game/Blueprint/Helpers/FunctionLibrary/BP_UsefullFunctions.CheckTargetClass` _currentsightactor "/Game/Blueprint/Player/BP_MainPlayer.BP_MainPlayer_C"))
  (bind _returnvalue_2 (`AIPerceptionSystem.GetSenseClassForStimulus` Stimulus))
  (if (== _returnvalue_2 "/Script/AIModule.AISense_Sight")
    (set `self.CurrentSightStimulus` Stimulus)
    (set `self.CurrentSightActor` Actor)
    (if _returnvalue
      (`/Game/Blueprint/Helpers/FunctionLibrary/BP_UsefullFunctions.SetBlackboardValueAsObject` (`self.Blackboard`) "Player" _returnobject)
      (`/Game/Blueprint/Helpers/FunctionLibrary/BP_UsefullFunctions.SetBlackboardValueAsVector` (`self.Blackboard`) "PlayerLocation" (`self.K2_GetActorLocation` _currentsightactor)))))

(fn `UserConstructionScript`)