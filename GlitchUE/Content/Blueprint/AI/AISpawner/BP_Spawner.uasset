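; AI spawner actor that spawns waves of AI at its own location and outlines its spawn mesh while activated.
; Spawn creates pawns with behavior trees picked at random from SpawnList, either all at once or spaced by SpawnDelay through ForLoopDelay.
; When a wave finishes spawning, EndSpawn increases the next wave's count by AddedAIToNextWave.
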(event `SetNewState`
  (params (State :type "/Game/Blueprint/Nexus/E_ObjectifState Enum" :default "NewEnumerator0"))
  (bind _output_get (set `self.State` State))
  (`/Game/Blueprint/Helpers/FunctionLibrary/BP_UsefullFunctions.OutlineElement` (select `/Game/Blueprint/Nexus/E_ObjectifState` _output_get :`NewEnumerator0` true) (`self.SpawnMesh`)))

(event `Spawn`
  (bind (_aiclass _behaviortree) (break `/Game/Blueprint/AI/AISpawner/F_SpawnAI` (`KismetArrayLibrary.Array_Random` (`self.SpawnList`))))
  (if (== (`self.SpawnDelay`) 0.0)
    (for _ (range (+ (`self.AIToSpawnForEachWaves`) 1))
      (`AIBlueprintHelperLibrary.SpawnAIFromClass` _aiclass _behaviortree (`self.K2_GetActorLocation`) (struct) false self :!label _label))
    (`self.EndSpawn`)
    (else
      (`/Game/Blueprint/Helpers/FunctionLibrary/BP_CustomMacros.ForLoopDelay` 0 (`self.AIToSpawnForEachWaves`) (`self.SpawnDelay`)
        (:`LoopBody`
          (goto _label))
        (:`Completed`
          (`self.EndSpawn`))))))

(event `EndSpawn`
  (set `self.AIToSpawnForEachWaves` (+ (`self.AddedAIToNextWave`) (`self.AIToSpawnForEachWaves`))))

(fn `UserConstructionScript`)