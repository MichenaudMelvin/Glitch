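; BP_WaveManager runs the game's timed waves, gathering all spawners and catalysers at BeginPlay and granting the player starting gold.
; StartWave toggles catalysers by their enable/disable wave numbers, then triggers every spawner in the required state.
; It re-calls itself after a delay, granting gold each time, until the final wave number is reached.
; A looping timer drives a debug-printed countdown to the next wave.
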(event `self.ReceiveBeginPlay`
  (bind _outactors (`GameplayStatics.GetAllActorsOfClass` "/Game/Blueprint/AI/AISpawner/BP_Spawner.BP_Spawner_C"))
  (set `self.SpawnerList` _outactors)
  (bind _outactors_2 (`GameplayStatics.GetAllActorsOfClass` "/Game/Blueprint/Nexus/BP_Catalyseur.BP_Catalyseur_C"))
  (set `self.CatalyseursList` _outactors_2)
  (bind _output_get (set `self.Player` (`/Game/Blueprint/Helpers/FunctionLibrary/BP_CallElements.CallBPMainPlayer`)))
  (`/Game/Blueprint/Player/BP_MainPlayer.GiveGolds` _output_get (`self.StartGolds`)))

(event `StartWave`
  (set `self.CurrentDisplayTime` (`self.WaveDuration`))
  (bind _returnvalue (`KismetSystemLibrary.K2_SetTimerDelegate` (`|CreateDelegate` :!event `ShowTimeWaveRemaning`) 0.1 true))
  (set `self.DisplayTimer` _returnvalue)
  (`/Engine/EditorBlueprintResources/StandardMacros.IncrementInt` (`self.CurrentWaveNumber`)
    (:`  `
      (`self.EnableOrDisableCatalyseurs`)
      (`self.Spawn`)
      (if (== (`self.CurrentWaveNumber`) (`self.WaveNumber`))
        (`/Game/Blueprint/Helpers/FunctionLibrary/BP_UsefullFunctions.Print` "les vagues sont terminées" true true (struct :`G` 0.321934 :`B` 1.0 :`A` 1.0) 10.0)
        (`KismetSystemLibrary.K2_ClearAndInvalidateTimerHandle` (`self.DisplayTimer`))
        (else
          (`KismetSystemLibrary.Delay` (`self.WaveDuration`))
          (`/Game/Blueprint/Player/BP_MainPlayer.GiveGolds` (`self.Player`) (`self.GivenGoldsAtWave`))
          (`self.StartWave`))))))

(event `ShowTimeWaveRemaning`
  (bind _output_get (set `self.CurrentDisplayTime` (- (`self.CurrentDisplayTime`) 0.1)))
  (`/Game/Blueprint/Helpers/FunctionLibrary/BP_UsefullFunctions.Print` (`KismetStringLibrary.Concat_StrStr` "Next wave in : " (`KismetStringLibrary.Conv_DoubleToString` _output_get)) true false (struct :`R` 0.218681 :`G` 0.385869 :`B` 1.0 :`A` 1.0) 0.1))

(event `self.ReceiveTick`
  (params (DeltaSeconds :type "Float (single-precision)"))
  (`/Game/Blueprint/Helpers/FunctionLibrary/BP_UsefullFunctions.Print` (`KismetStringLibrary.Concat_StrStr` "Current wave : " (`KismetStringLibrary.Conv_IntToString` (`self.CurrentWaveNumber`))) false false (struct :`R` 0.404428 :`B` 1.0 :`A` 1.0) 0.0))

(fn `EnableOrDisableCatalyseurs`
  (for _array_element (`self.CatalyseursList`)
    (if (== (`self.CurrentWaveNumber`) (`/Game/Blueprint/Nexus/BP_Catalyseur.EnableAtWave` _array_element))
      (`/Game/Blueprint/Nexus/BP_AbstractObjectif.ActiveObject` _array_element)
      (elif (== (`self.CurrentWaveNumber`) (`/Game/Blueprint/Nexus/BP_Catalyseur.DisableAtWave` _array_element))
        (`/Game/Blueprint/Nexus/BP_AbstractObjectif.DesactivateObject` _array_element))))
  (return))

(fn `Spawn`
  (for _array_element (`self.SpawnerList`)
    (if (`|EnumEquality` (`/Game/Blueprint/AI/AISpawner/BP_Spawner.State` _array_element) "NewEnumerator0")
      (`/Game/Blueprint/AI/AISpawner/BP_Spawner.Spawn` _array_element)))
  (return))

(fn `UserConstructionScript`)