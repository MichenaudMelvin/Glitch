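; BP_FocusCatalyseurController is an AI controller for enemies that focus on Catalyseurs and the Nexus.
; On BeginPlay it caches all Catalyseurs and seeds the blackboard with the first Nexus's location, an attack distance and a Catalyseurs-left flag.
; It extends the parent's perception update, writing a sighted Nexus or, failing that, a sighted Catalyseur to its blackboard key as a target.
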(event `self.ReceiveBeginPlay`
  (`parent.ReceiveBeginPlay`)
  (bind _outactors (`GameplayStatics.GetAllActorsOfClass` "/Game/Blueprint/Nexus/BP_Catalyseur.BP_Catalyseur_C"))
  (set `self.CatalyseurList` _outactors)
  (bind _outactors_2 (`GameplayStatics.GetAllActorsOfClass` "/Game/Blueprint/Nexus/BP_Nexus.BP_Nexus_C"))
  (`/Game/Blueprint/Helpers/FunctionLibrary/BP_UsefullFunctions.SetBlackboardValueAsVector` (`self.Blackboard`) "NexusLocation" (`self.K2_GetActorLocation` (`|GetArrayItem` _outactors_2)))
  (`/Game/Blueprint/Helpers/FunctionLibrary/BP_UsefullFunctions.SetBlackboardValueAsBool` (`self.Blackboard`) "AnyCatalyseursLeft" true)
  (`/Game/Blueprint/Helpers/FunctionLibrary/BP_UsefullFunctions.SetBlackboardValueAsFloat` (`self.Blackboard`) "AttackDistance" 200.0))

(event `self.TargetPerceptionUpdatedEvent`
  (params (Actor :type "Actor Object Reference") (Stimulus :type "AIStimulus Structure"))
  (bind (_returnvalue _returnobject) (`/Game/Blueprint/Helpers/FunctionLibrary/BP_UsefullFunctions.CheckTargetClass` (`self.CurrentSightActor`) "/Game/Blueprint/Nexus/BP_Nexus.BP_Nexus_C"))
  (bind (_returnvalue_2 _returnobject_2) (`/Game/Blueprint/Helpers/FunctionLibrary/BP_UsefullFunctions.CheckTargetClass` (`self.CurrentSightActor`) "/Game/Blueprint/Nexus/BP_Catalyseur.BP_Catalyseur_C"))
  (`parent.TargetPerceptionUpdatedEvent` Actor Stimulus)
  (if _returnvalue
    (`/Game/Blueprint/Helpers/FunctionLibrary/BP_UsefullFunctions.SetBlackboardValueAsObject` (`self.Blackboard`) "Nexus" _returnobject)
    (elif _returnvalue_2
      (`/Game/Blueprint/Helpers/FunctionLibrary/BP_UsefullFunctions.SetBlackboardValueAsObject` (`self.Blackboard`) "CurrentFocusedCatalyseur" _returnobject_2))))

(fn `UserConstructionScript`
  (`parent.UserConstructionScript`))