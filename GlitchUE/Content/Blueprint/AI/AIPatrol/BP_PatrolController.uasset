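; AI controller for patrolling enemies that turns sight of the player into a gradual detection before alerting the level.
; Seeing MainPlayer starts a looping investigate timer, shows a temporary sight widget and sets Blackboard Investigate.
; Each tick updates the widget and investigation location, raising or lowering elapsed time with visibility.
; Full detection writes the player to the Blackboard and sets Alerted; either limit ends investigation.
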(event `self.ReceiveBeginPlay`
  (`parent.ReceiveBeginPlay`))

(event `self.PerceptionUpdate`
  (params (Actor :type "Actor Object Reference") (Stimulus :type "AIStimulus Structure"))
  (`parent.PerceptionUpdate` Actor Stimulus)
  (bind _returnvalue (`AIPerceptionSystem.GetSenseClassForStimulus` Stimulus))
  (if (== _returnvalue "/Script/AIModule.AISense_Sight")
    (if (`/Game/Blueprint/Helpers/FunctionLibrary/BP_UsefullFunctions.CheckParentClass` Actor "/Script/GlitchUE.MainPlayer")
      (if (not (`KismetSystemLibrary.K2_IsTimerActiveHandle` (`self.InvestigateTimer`)))
        (bind _returnvalue_2 (`KismetSystemLibrary.K2_SetTimerDelegate` (`|CreateDelegate` :!event `Investigate`) 0.1 true))
        (set `self.InvestigateTimer` _returnvalue_2)
        (`SceneComponent.SetVisibility` (`/Game/Blueprint/AI/BP_MainAICharacter.TEMP_SightWidget` (`self.AICharacter`)) true false)
        (`/Game/Blueprint/Helpers/FunctionLibrary/BP_UsefullFunctions.SetBlackboardValueAsBool` (`self.Blackboard`) "Investigate" true)))))

(event `Investigate`
  (bind _currentsightactor (`self.CurrentSightActor`))
  (`/Game/Blueprint/AI/Temp/WBP_SightIndication.TEMP_Time` (cast `/Game/Blueprint/AI/Temp/WBP_SightIndication` (`WidgetComponent.GetWidget` (`/Game/Blueprint/AI/BP_MainAICharacter.TEMP_SightWidget` (`self.AICharacter`))) :!pure true) (/ (* 100 (`self.InvestigateTimeElapsed`)) 2.0))
  (`/Game/Blueprint/Helpers/FunctionLibrary/BP_UsefullFunctions.SetBlackboardValueAsVector` (`self.Blackboard`) "InvestigationLocation" (`self.K2_GetActorLocation` (`self.CurrentSightActor`)))
  (if (`self.IsPlayerStillInSight`)
    (set `self.InvestigateTimeElapsed` (+ (`self.InvestigateTimeElapsed`) 0.1))
    (if (>= (`self.InvestigateTimeElapsed`) 2.0)
      (`/Game/Blueprint/Helpers/FunctionLibrary/BP_UsefullFunctions.SetBlackboardValueAsObject` (`self.Blackboard`) "Player" _currentsightactor)
      (`/Game/Blueprint/Helpers/FunctionLibrary/BP_UsefullFunctions.SetBlackboardValueAsVector` (`self.Blackboard`) "PlayerLocation" (`self.K2_GetActorLocation` _currentsightactor))
      (`GlitchUEGameMode.SetLevelState` (`/Game/Blueprint/Helpers/FunctionLibrary/BP_CallElements.CallMainGamemode`) "Alerted")
      (`KismetSystemLibrary.K2_ClearAndInvalidateTimerHandle` (`self.InvestigateTimer`) :!label _label)
      (`SceneComponent.SetVisibility` (`/Game/Blueprint/AI/BP_MainAICharacter.TEMP_SightWidget` (`self.AICharacter`)) false false)
      (`/Game/Blueprint/Helpers/FunctionLibrary/BP_UsefullFunctions.SetBlackboardValueAsBool` (`self.Blackboard`) "Investigate"))
    (else
      (set `self.InvestigateTimeElapsed` (- (`self.InvestigateTimeElapsed`) 0.1))
      (if (<= (`self.InvestigateTimeElapsed`) 0.0)
        (goto _label)))))

(fn `UserConstructionScript`
  (`parent.UserConstructionScript`))