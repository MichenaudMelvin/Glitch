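; Base AI character that shows its current health as text and drives a temporary sight indicator widget.
; On BeginPlay it caches the AI controller and blackboard after a short delay, then stores its spawn location as OriginalPosition.
; HealthComp damage events refresh the text, and Sight events feed investigate percentage to the widget.
; Tick debug-prints IsStun; the interact event is empty, with unseen-player kill logic left disconnected.
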(event `self.ReceiveBeginPlay`
  (`self.UpdateHealth`)
  (`KismetSystemLibrary.Delay` 0.2)
  (bind _output_get (set `self.AIController` (cast `/Game/Blueprint/AI/BP_MainAIController` (`self.GetController`) :!pure true)))
  (bind _output_get_2 (set `self.Blackboard` (`AIBlueprintHelperLibrary.GetBlackboard` _output_get)))
  (`/Game/Blueprint/Helpers/FunctionLibrary/BP_UsefullFunctions.SetBlackboardValueAsVector` _output_get_2 "OriginalPosition" (`self.K2_GetActorLocation`)))

(event `self.ReceiveTick`
  (params (DeltaSeconds :type "Float (single-precision)"))
  (bind _blackboard (`self.Blackboard`))
  (`parent.ReceiveTick` DeltaSeconds)
  (`/Engine/EditorBlueprintResources/StandardMacros.IsValid` _blackboard
    (:`Is Valid`
      (`/Game/Blueprint/Helpers/FunctionLibrary/BP_UsefullFunctions.Print` (`KismetStringLibrary.Concat_StrStr` "IsStun : " (`KismetStringLibrary.Conv_BoolToString` (`/Game/Blueprint/Helpers/FunctionLibrary/BP_UsefullFunctions.GetBlackboardValueAsBool` _blackboard "IsStun"))) true false (struct :`R` 0.045752 :`G` 0.143075 :`B` 1.0 :`A` 1.0) 0.0))))

(event `self.Interactable.OnInteract`
  (params (MainPlayerController :type "MainPlayerController Object Reference") (MainPlayer :type "MainPlayer Object Reference")))

(event `self.HealthComp.OnReciveDamages`
  (`self.UpdateHealth`))

(event `self.Sight.OnSightPlayer`
  (params (InvestigateTimePercent :type "Float (single-precision)"))
  (`/Game/Blueprint/AI/Temp/WBP_SightIndication.TEMP_Time` (cast `/Game/Blueprint/AI/Temp/WBP_SightIndication` (`WidgetComponent.GetWidget` (`self.TEMP_SightWidget`)) :!pure true) InvestigateTimePercent))

(event `self.Sight.OnLooseSightPlayer`
  (params (InvestigateTimePercent :type "Float (single-precision)"))
  (`/Game/Blueprint/AI/Temp/WBP_SightIndication.TEMP_Time` (cast `/Game/Blueprint/AI/Temp/WBP_SightIndication` (`WidgetComponent.GetWidget` (`self.TEMP_SightWidget`)) :!pure true) InvestigateTimePercent))

(fn `UpdateHealth`
  (`TextRenderComponent.K2_SetText` (`self.ShowHealth`) (`KismetTextLibrary.Conv_DoubleToText` (`HealthComponent.CurrentHealth` (`self.HealthComp`)) "HalfToEven"))
  (return))

(fn `UserConstructionScript`)