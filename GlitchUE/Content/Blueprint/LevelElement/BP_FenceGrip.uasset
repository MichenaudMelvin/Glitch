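; BP_FenceGrip is a level element that switches its particle effects between Tech and Med versions when a dissolver reaches it.
; DissolverTrigger overlaps filter for BP_Dissolver actors: entering starts MedEmitter and stops TechEmitter, and exiting reverses this.
; On entry it also clears TechEmitter's PlayOnLoad, so an instant dissolver does not show the Tech effect at start.
; The construction script only calls the parent's.
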(event `self.DissolverTrigger.OnComponentBeginOverlap`
  (params (OverlappedComponent :type "PrimitiveComponent Object Reference") (OtherActor :type "Actor Object Reference") (OtherComp :type "PrimitiveComponent Object Reference") (OtherBodyIndex :type Integer) (bFromSweep :type Boolean) (SweepResult :type "HitResult Structure (by ref)"))
  (if (`/Game/Blueprint/Helpers/FunctionLibrary/BP_UsefullFunctions.CheckParentClass` OtherActor "/Game/Blueprint/FX/BP_Dissolver.BP_Dissolver_C")
    (`self.OnDissolverEnter`)))

(event `self.DissolverTrigger.OnComponentEndOverlap`
  (params (OverlappedComponent :type "PrimitiveComponent Object Reference") (OtherActor :type "Actor Object Reference") (OtherComp :type "PrimitiveComponent Object Reference") (OtherBodyIndex :type Integer))
  (if (`/Game/Blueprint/Helpers/FunctionLibrary/BP_UsefullFunctions.CheckParentClass` OtherActor "/Game/Blueprint/FX/BP_Dissolver.BP_Dissolver_C")
    (`self.OnDissolverExit`)))

(event `OnDissolverEnter`
  (bind _techemitter (`self.TechEmitter`))
  (`PopcornFXEmitterComponent.StartEmitter` (`self.MedEmitter`))
  (set `PopcornFXEmitterComponent.bPlayOnLoad` false _techemitter) ; This is used for instant MedDissolver, Otherwise the FX will play at start
  (`PopcornFXEmitterComponent.StopEmitter` _techemitter false))

(event `OnDissolverExit`
  (`PopcornFXEmitterComponent.StartEmitter` (`self.TechEmitter`))
  (`PopcornFXEmitterComponent.StopEmitter` (`self.MedEmitter`) false))

(fn `UserConstructionScript`
  (`parent.UserConstructionScript`))