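; Light element Blueprint variant with candles, which toggles candle emitters in response to dissolver enter and exit events.
; It extends the parent's dissolver handling, then loops over CandleList to start each emitter on enter and stop it on exit.
; The construction script only calls the parent's.
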(event `self.OnDissolverEnter`
  (`parent.OnDissolverEnter`)
  (for _array_element (`self.CandleList`)
    (`PopcornFXEmitterComponent.StartEmitter` _array_element)))

(event `self.OnDissolverExit`
  (`parent.OnDissolverExit`)
  (for _array_element (`self.CandleList`)
    (`PopcornFXEmitterComponent.StopEmitter` _array_element false)))

(fn `UserConstructionScript`
  (`parent.UserConstructionScript`))