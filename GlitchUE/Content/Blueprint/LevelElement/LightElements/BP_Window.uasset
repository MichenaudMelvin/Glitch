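; BP_Window is a window light element whose spotlight changes brightness when a BP_Dissolver enters or leaves its box trigger.
; It starts play at the TECH intensity, while the construction script sets the MED intensity.
; Box overlaps filtered by parent class play or reverse a timeline that lerps the light from TECH to MED intensity and back.
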(event `self.ReceiveBeginPlay`
  (`LightComponent.SetIntensity` (`self.SpotLight`) (`self.TECHIntensity`)))

(event `self.Box.OnComponentBeginOverlap`
  (params (OverlappedComponent :type "PrimitiveComponent Object Reference") (OtherActor :type "Actor Object Reference") (OtherComp :type "PrimitiveComponent Object Reference") (OtherBodyIndex :type Integer) (bFromSweep :type Boolean) (SweepResult :type "HitResult Structure (by ref)"))
  (if (`/Game/Blueprint/Helpers/FunctionLibrary/BP_UsefullFunctions.CheckParentClass` OtherActor "/Game/Blueprint/FX/BP_Dissolver.BP_Dissolver_C")
    (`self.OnEnter`)))

(event `self.Box.OnComponentEndOverlap`
  (params (OverlappedComponent :type "PrimitiveComponent Object Reference") (OtherActor :type "Actor Object Reference") (OtherComp :type "PrimitiveComponent Object Reference") (OtherBodyIndex :type Integer))
  (if (`/Game/Blueprint/Helpers/FunctionLibrary/BP_UsefullFunctions.CheckParentClass` OtherActor "/Game/Blueprint/FX/BP_Dissolver.BP_Dissolver_C")
    (`self.OnExit`)))

(event `OnEnter`
  (bind (_direction _value) (`Timeline|LightIntensityTimeline` :!label _label)
    (:`Update`
      (`LightComponent.SetIntensity` (`self.SpotLight`) (`KismetMathLibrary.Lerp` (`self.TECHIntensity`) (`self.MEDIntensity`) _value)))))

(event `OnExit`
  (goto _label :!via `Reverse`))

(fn `UserConstructionScript`
  (`LightComponent.SetIntensity` (`self.SpotLight`) (`self.MEDIntensity`)))