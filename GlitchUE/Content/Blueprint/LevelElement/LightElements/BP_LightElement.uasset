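; BP_LightElement is a level light that shifts its color temperature while a BP_Dissolver actor is inside its Box trigger.
; On begin overlap, LightTempTimeline plays and lerps the PointLight temperature from LightTempMax toward LightTempMin.
; On end overlap, the same timeline reverses to blend the temperature back, with both events filtered by a parent-class check.
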(event `self.Box.OnComponentBeginOverlap`
  (params (OverlappedComponent :type "PrimitiveComponent Object Reference") (OtherActor :type "Actor Object Reference") (OtherComp :type "PrimitiveComponent Object Reference") (OtherBodyIndex :type Integer) (bFromSweep :type Boolean) (SweepResult :type "HitResult Structure (by ref)"))
  (if (`/Game/Blueprint/Helpers/FunctionLibrary/BP_UsefullFunctions.CheckParentClass` OtherActor "/Game/Blueprint/FX/BP_Dissolver.BP_Dissolver_C")
    (bind (_direction _value) (`Timeline|LightTempTimeline` :!label _label)
      (:`Update`
        (`LightComponent.SetTemperature` (`self.PointLight`) (`KismetMathLibrary.Lerp` (`self.LightTempMax`) (`self.LightTempMin`) _value))))))

(event `self.Box.OnComponentEndOverlap`
  (params (OverlappedComponent :type "PrimitiveComponent Object Reference") (OtherActor :type "Actor Object Reference") (OtherComp :type "PrimitiveComponent Object Reference") (OtherBodyIndex :type Integer))
  (if (`/Game/Blueprint/Helpers/FunctionLibrary/BP_UsefullFunctions.CheckParentClass` OtherActor "/Game/Blueprint/FX/BP_Dissolver.BP_Dissolver_C")
    (goto _label :!via `Reverse`)))

(fn `UserConstructionScript`
  (`parent.UserConstructionScript`))