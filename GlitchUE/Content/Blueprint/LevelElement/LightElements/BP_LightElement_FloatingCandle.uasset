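; BP_LightElement_FloatingCandle is a light element level Blueprint for a group of floating candles.
; On BeginPlay it runs the parent logic, then fills CandleList with its ten PkFireCandle references.
; The construction script only calls the parent, and this graph holds no floating or lighting logic of its own.
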(event `self.ReceiveBeginPlay`
  (`parent.ReceiveBeginPlay`)
  (set `self.CandleList` (`|MakeArray` (`self.Pk_Fire_Candle`) (`self.Pk_Fire_Candle1`) (`self.Pk_Fire_Candle2`) (`self.Pk_Fire_Candle3`) (`self.Pk_Fire_Candle4`) (`self.Pk_Fire_Candle5`) (`self.Pk_Fire_Candle6`) (`self.Pk_Fire_Candle7`) (`self.Pk_Fire_Candle8`) (`self.Pk_Fire_Candle9`))))

(fn `UserConstructionScript`
  (`parent.UserConstructionScript`))