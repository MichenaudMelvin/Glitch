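; Abstract base door that players toggle by interaction and AI characters open on reaching its smart nav link.
; A timeline scaled by OpenDoorTime plays or reverses, feeding an empty OpenDoorUpdate hook for the door motion.
; On finish it flips IsOpen, switching the smart link and nav modifier area to match.
; AI arrivals, gated by a DoOnce, set the DoingExternalActions blackboard flag, clearing it after opening a closed door.
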(event `self.ReceiveBeginPlay`
  (`parent.ReceiveBeginPlay`)
  (`InteractableComponent.AddInteractables` (`self.DoorInteraction`) (`|MakeArray` (`self.MED_Door`) (`self.TECH_Door`) :!type "PrimitiveComponent Object Reference"))
  (bind _output_get (set `self.NavLink` (cast `NavLinkProxy` (`ChildActorComponent.ChildActor` (`self.NavLinkProxy`)) :!pure true)))
  (add `NavLinkProxy.OnSmartLinkReached` _output_get (`|CreateDelegate` :!event `LinkReached`))
  (`TimelineComponent.SetPlayRate` (`self.OpenDoorTimeline`) (/ 1.0 (`self.OpenDoorTime`))))

(event `self.DoorInteraction.OnInteract`
  (params (MainPlayerController :type "MainPlayerController Object Reference") (MainPlayer :type "MainPlayer Object Reference"))
  (set `self.CurrentCharacterOpenningDoor` MainPlayer)
  (if (not (`TimelineComponent.IsPlaying` (`self.OpenDoorTimeline`)))
    (`self.OpenAndCloseDoor`)))

(event `OpenAndCloseDoor`
  (if (`self.IsOpen`)
    (`self.CloseDoor`)
    (else
      (`self.OpenDoor`))))

(event `OpenDoor`
  (bind (_direction _alpha) (`Timeline|OpenDoorTimeline` :!label _label)
    (:`Update`
      (`self.OpenDoorUpdate` _alpha))
    (:`Finished`
      (`self.OpenDoorFinished`))))

(event `OpenDoorEditor`
  ;[0.5 0.5 1] Editor
)

(event `CloseDoor`
  (goto _label :!via `Reverse`))

(event `CloseDoorEditor`
  ;[0.5 0.5 1] Editor
)

(event `OpenDoorUpdate`
  (params (Alpha :type "Float (double-precision)")))

(event `OpenDoorFinished`
  (bind _returnvalue (not (`self.IsOpen`)))
  (bind _output_get (set `self.IsOpen` _returnvalue))
  (`NavLinkProxy.SetSmartLinkEnabled` (`self.NavLink`) _returnvalue)
  (`NavModifierComponent.SetAreaClass` (`self.NavModifier`) (select `bool` _output_get :`false` "/Script/NavigationSystem.NavArea_Null" :`true` "/Script/NavigationSystem.NavArea_Default" :!type "NavArea Class Reference")))

(event `LinkReached`
  (params (MovingActor :type "Actor Object Reference") (DestinationPoint :type "Vector Structure (by ref)"))
  (bind _asmain_aicharacter (cast `MainAICharacter` MovingActor :!pure true))
  (`/Engine/EditorBlueprintResources/StandardMacros.DoOnce` false :!label _label_2
    (:`Completed`
      (`/Game/Blueprint/Helpers/FunctionLibrary/BP_UsefullFunctions.SetBlackboardValueAsBool` (`MainAICharacter.Blackboard` _asmain_aicharacter) "DoingExternalActions" true)
      (if (not (`self.IsOpen`))
        (set `self.CurrentCharacterOpenningDoor` _asmain_aicharacter)
        (`self.OpenDoor`)
        (`KismetSystemLibrary.Delay` (`UsefullFunctions.GetTimelineDuration` (`self.OpenDoorTimeline`)))
        (`/Game/Blueprint/Helpers/FunctionLibrary/BP_UsefullFunctions.SetBlackboardValueAsBool` (`MainAICharacter.Blackboard` _asmain_aicharacter) "DoingExternalActions")
        (`KismetSystemLibrary.Delay` 1.0))
      (`self.ResetLinkReached`))))

(event `ResetLinkReached`
  (goto _label_2 :!via `Reset`))

(fn `UserConstructionScript`
  (`parent.UserConstructionScript`))