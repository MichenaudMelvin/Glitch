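; Interactable door actor that swings its MEDDoor and TECHDoor meshes together when the player interacts with either.
; A timeline plays or reverses the 90-degree swing, ignoring interaction while running.
; A dot product between MEDMesh and player forward vectors picks the opening direction.
; Editor events pose the door open either way or closed, and BeginPlay infers state and direction from that placed rotation.
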(event `self.ReceiveBeginPlay`
  (bind _relativerotation (`SceneComponent.RelativeRotation` (`self.MED_Door`)))
  (`parent.ReceiveBeginPlay`)
  (`BlueprintSetLibrary.Set_AddItems` (`/Game/Blueprint/Interactables/AC_Interactable.InteractableComponentSet` (`self.DoorInteraction`)) (`|MakeArray` (`self.MED_Door`) (`self.TECH_Door`) :!type "PrimitiveComponent Object Reference"))
  (set `self.IsOpen` (not (== _relativerotation (struct))))
  (set `self.RotationFactor` (select `bool` (and (== _relativerotation (struct :`Yaw` 90.0)) (`self.IsOpen`)) :`false` -1 :`true` 1))
  (`TimelineComponent.SetPlaybackPosition` (`self.OpenDoorTimeline`) (select `bool` (`self.IsOpen`) :`true` 1.0 :!type "Float (single-precision)") false true))

(event `self.DoorInteraction.OnInteract`
  (params (BPMainPlayerController :type "/Game/Blueprint/Player/Controllers/BP_PC_MainPlayerController Object Reference") (BPMainPlayer :type "/Game/Blueprint/Player/BP_MainPlayer Object Reference"))
  (set `self.Player` BPMainPlayer)
  (if (not (`TimelineComponent.IsPlaying` (`self.OpenDoorTimeline`)))
    (`self.OpenAndCloseDoor`)))

(event `OpenAndCloseDoor`
  (if (`self.IsOpen`)
    (`self.CloseDoor`)
    (else
      (set `self.RotationFactor` (`self.Select Rotation Factor`))
      (`self.OpenDoor`))))

(event `OpenDoor`
  (bind (_direction _rotationalpha) (`Timeline|OpenDoorTimeline` :!label _label)
    (:`Update`
      (bind _returnvalue (`KismetMathLibrary.RLerp` (struct) (struct :`Yaw` 90.0) (* (`self.RotationFactor`) _rotationalpha)))
      (`SceneComponent.K2_SetRelativeRotation` (`self.MED_Door`) _returnvalue false false)
      (`SceneComponent.K2_SetRelativeRotation` (`self.TECH_Door`) _returnvalue false false))
    (:`Finished`
      (set `self.IsOpen` (not (`self.IsOpen`))))))

(event `CloseDoor`
  (goto _label :!via `Reverse`))

(event `OpenDoorEditor`
  ;[0.5 0.5 1] Editor
  (`/Engine/EditorBlueprintResources/StandardMacros.FlipFlop`
    (:`A`
      (`SceneComponent.K2_SetRelativeRotation` (`self.MED_Door`) (struct :`Yaw` 90.0) false false)
      (`SceneComponent.K2_SetRelativeRotation` (`self.TECH_Door`) (struct :`Yaw` 90.0) false false))
    (:`B`
      (`SceneComponent.K2_SetRelativeRotation` (`self.MED_Door`) (struct :`Yaw` -90.0) false false)
      (`SceneComponent.K2_SetRelativeRotation` (`self.TECH_Door`) (struct :`Yaw` -90.0) false false))))

(event `CloseDoorEditor`
  ;[0.5 0.5 1] Editor
  (`SceneComponent.K2_SetRelativeRotation` :`self` (`self.MED_Door`))
  (`SceneComponent.K2_SetRelativeRotation` :`self` (`self.TECH_Door`)))

(fn `Select Rotation Factor`
  (returns (Factor :type Integer))
  (return (select `bool` (>= (`KismetMathLibrary.Dot_VectorVector` (`SceneComponent.GetForwardVector` (`self.MED_Mesh`)) (`SceneComponent.GetForwardVector` (`Character.CapsuleComponent` (`self.Player`)))) 0.0) :`false` 1 :`true` -1)))

(fn `UserConstructionScript`
  (`parent.UserConstructionScript`))