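; BP_LightElement is a level element whose point light changes color temperature when a dissolver touches it.
; Overlap events on MED_Mesh check whether the other actor derives from BP_Dissolver.
; A dissolver beginning overlap shifts PointLight to a warm temperature, and one ending overlap sets it to a cool one.
; The construction script only calls its parent's version.
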(event `self.MED_Mesh.OnComponentBeginOverlap`
  (params (OverlappedComponent :type "PrimitiveComponent Object Reference") (OtherActor :type "Actor Object Reference") (OtherComp :type "PrimitiveComponent Object Reference") (OtherBodyIndex :type Integer) (bFromSweep :type Boolean) (SweepResult :type "HitResult Structure (by ref)"))
  (if (`/Game/Blueprint/Helpers/FunctionLibrary/BP_UsefullFunctions.CheckParentClass` OtherActor "/Game/Blueprint/FX/BP_Dissolver.BP_Dissolver_C")
    (`LightComponent.SetTemperature` (`self.PointLight`) 2500.0)))

(event `self.MED_Mesh.OnComponentEndOverlap`
  (params (OverlappedComponent :type "PrimitiveComponent Object Reference") (OtherActor :type "Actor Object Reference") (OtherComp :type "PrimitiveComponent Object Reference") (OtherBodyIndex :type Integer))
  (if (`/Game/Blueprint/Helpers/FunctionLibrary/BP_UsefullFunctions.CheckParentClass` OtherActor "/Game/Blueprint/FX/BP_Dissolver.BP_Dissolver_C")
    (`LightComponent.SetTemperature` (`self.PointLight`) 9500.0)))

(fn `UserConstructionScript`
  (`parent.UserConstructionScript`))