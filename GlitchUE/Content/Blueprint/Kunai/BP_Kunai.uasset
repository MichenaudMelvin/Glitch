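; Kunai projectile that serves as the main player's mark, with a computed teleport location and a Niagara beam.
; It registers with the character on BeginPlay, flies when launched and sticks on hit.
; Looping timers run during flight; a reset returns it to its original location, clears the beam and rebinds the controller's glitch event.
; Vertical traces offset the teleport point by capsule half-height from nearby floors or ceilings.
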(event `self.ReceiveBeginPlay`
  (`self.StopProjectile`)
  (set `self.OriginalLocation` (`self.K2_GetActorLocation`))
  (bind _output_get (set `self.Character` (`/Game/Blueprint/Helpers/FunctionLibrary/BP_CallElements.CallBPMainPlayer`)))
  (set `/Game/Blueprint/Player/BP_MainPlayer.Mark` self _output_get))

(event `self.ReceiveHit`
  (params (MyComp :type "PrimitiveComponent Object Reference") (Other :type "Actor Object Reference") (OtherComp :type "PrimitiveComponent Object Reference") (bSelfMoved :type Boolean) (HitLocation :type "Vector Structure") (HitNormal :type "Vector Structure") (NormalImpulse :type "Vector Structure") (Hit :type "HitResult Structure (by ref)"))
  (`self.PlaceMark`))

(event `AttachBeamEndToPlayer`
  ;[1 1 1] Manage beam points
  (`FXSystemComponent.SetVectorParameter` (`self.Niagara`) "BeamEnd" (`self.K2_GetActorLocation` (`self.Character`))))

(event `ResetBeamEnd`
  ;[1 1 1] Manage beam points
  (`FXSystemComponent.SetVectorParameter` (`self.Niagara`) "BeamEnd" (0.0 0.0 0.0)))

(event `LaunchMark`
  (params (StartTransform :type "Transform Structure"))
  ;[1 1 1] Manage mark movement
  (`self.K2_SetActorTransform` StartTransform)
  (set `self.LaunchLocation` (.location StartTransform))
  (`self.StartProjectile`)
  (bind _returnvalue (`KismetSystemLibrary.K2_SetTimerDelegate` (`|CreateDelegate` :!event `CheckDistance`) 0.0001 true))
  (set `self.DistanceTimer` _returnvalue)
  (bind _returnvalue_2 (`KismetSystemLibrary.K2_SetTimerDelegate` (`|CreateDelegate` :!event `AttachBeamEndToPlayer`) 0.0001 true))
  (set `self.BeamTickTimer` _returnvalue_2))

(event `PlaceMark`
  ;[1 1 1] Manage mark movement
  (`self.StopProjectile`)
  (set `self.IsMarkPlaced` true)
  (`KismetSystemLibrary.K2_ClearAndInvalidateTimerHandle` (`self.DistanceTimer`)))

(event `ResetMark`
  (bind _mainplayercontroller (`/Game/Blueprint/Player/BP_MainPlayer.MainPlayerController` (`self.Character`)))
  ;[1 1 1] Manage mark movement
  (clear `/Game/Blueprint/Player/Controllers/BP_PC_MainPlayerController.OnUseGlitch` _mainplayercontroller)
  (add `/Game/Blueprint/Player/Controllers/BP_PC_MainPlayerController.OnUseGlitch` _mainplayercontroller (`|CreateDelegate` (`self.Character`) :!event `LaunchMark`))
  (`KismetSystemLibrary.K2_ClearAndInvalidateTimerHandle` (`self.DistanceTimer`))
  (`KismetSystemLibrary.K2_ClearAndInvalidateTimerHandle` (`self.BeamTickTimer`))
  (`self.K2_SetActorLocation` (`self.OriginalLocation`))
  (`self.StopProjectile`)
  (set `self.IsMarkPlaced` false)
  (`self.ResetBeamEnd`))

(fn `CheckDistance`
  (if (and (>= (`self.GetDistanceToLaunchPoint`) (`self.MaxDistance`)) (not (`self.IsMarkPlaced`)))
    (`self.ResetMark`)
    (return)
    (else
      (return))))

(fn `GetDistanceToLaunchPoint`
  (returns (DistanceValue :type "Float (double-precision)"))
  (return (`KismetMathLibrary.Vector_Distance` (`self.LaunchLocation`) (`self.K2_GetActorLocation`))))

(fn `GetTPLocation`
  (returns (Location :type "Vector Structure"))
  (bind (_impactpoint _returnvalue) (`self.LocationTrace` (* -1 (`CapsuleComponent.CapsuleHalfHeight` (`Character.CapsuleComponent` (`self.Character`)))))) ; Check si il y a quelque chose en dessous de la marque
  (if _returnvalue
    (return (`/Game/Blueprint/Helpers/FunctionLibrary/BP_UsefullFunctions.AddToVector` _impactpoint 0.0 0.0 (`CapsuleComponent.CapsuleHalfHeight` (`Character.CapsuleComponent` (`self.Character`)))))
    (else
      (bind (_impactpoint_2 _returnvalue_2) (`self.LocationTrace` (`CapsuleComponent.CapsuleHalfHeight` (`Character.CapsuleComponent` (`self.Character`))))) ; Check si il y a quelque chose au dessus de la marque
      (if _returnvalue_2
        (return (`/Game/Blueprint/Helpers/FunctionLibrary/BP_UsefullFunctions.AddToVector` _impactpoint_2 0.0 0.0 (* -1 (`CapsuleComponent.CapsuleHalfHeight` (`Character.CapsuleComponent` (`self.Character`))))))
        (else
          (return (`self.K2_GetActorLocation`)))))))

(fn `LocationTrace`
  (params (UpTraceValue :type "Float (double-precision)"))
  (returns (ImpactPoint :type "Vector Structure") (ReturnValue :type Boolean))
  (bind _returnvalue (`self.K2_GetActorLocation`))
  (bind (_outhit _returnvalue_2) (`KismetSystemLibrary.LineTraceSingle` _returnvalue (`/Game/Blueprint/Helpers/FunctionLibrary/BP_UsefullFunctions.AddToVector` _returnvalue 0.0 0.0 (`local.UpTraceValue`)) "TraceTypeQuery1"))
  (return (`.ImpactPoint` (`GameplayStatics.BreakHitResult` _outhit)) _returnvalue_2))

(fn `StartProjectile`
  (bind _projectilemovement (`self.ProjectileMovement`))
  (`ProjectileMovementComponent.SetVelocityInLocalSpace` _projectilemovement (`KismetMathLibrary.MakeVector` (`ProjectileMovementComponent.MaxSpeed` (`self.ProjectileMovement`))))
  (set `ProjectileMovementComponent.ProjectileGravityScale` 1.0 _projectilemovement)
  (return))

(fn `StopProjectile`
  (bind _projectilemovement (`self.ProjectileMovement`))
  (`ProjectileMovementComponent.SetVelocityInLocalSpace` _projectilemovement (0.0 0.0 0.0))
  (set `ProjectileMovementComponent.ProjectileGravityScale` 0.0 _projectilemovement)
  (return))

(fn `UserConstructionScript`)