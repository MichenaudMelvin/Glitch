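; Nexus actor that drives the level's BP_Dissolver radial dissolve from its health and from activated catalysts.
; The construction script moves the first found dissolver onto the Nexus and refreshes its shader FX.
; Damage dissolves to a radius scaled by current health.
; Its own activation, after a short delay, dissolves to the distance of the farthest activated BP_Catalyseur, picked by distance-sorting those cached at BeginPlay.
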(event `self.ReceiveBeginPlay`
  (`parent.ReceiveBeginPlay`)
  (bind _outactors (`GameplayStatics.GetAllActorsOfClass` "/Game/Blueprint/FX/BP_Dissolver.BP_Dissolver_C"))
  (set `self.Dissolver` (`|GetArrayItem` _outactors))
  (bind _outactors_2 (`GameplayStatics.GetAllActorsOfClass` "/Game/Blueprint/Nexus/BP_Catalyseur.BP_Catalyseur_C"))
  (for _array_element _outactors_2
    (`BlueprintSetLibrary.Set_Add` (`self.CatalyseurList`) _array_element)))

(event `self.HealthComp.OnReciveDamages`
  (bind _healthcomp (`self.HealthComp`))
  (`/Game/Blueprint/FX/BP_Dissolver.DissolveTo` (`self.Dissolver`) (/ (* (/ (* (`HealthComponent.CurrentHealth` _healthcomp) (`HealthComponent.MaxHealth` _healthcomp)) 100.0) (`/Game/Blueprint/FX/BP_Dissolver.Radius` (`self.Dissolver`))) 100.0)))

(event `self.ActivableComp.OnActivated`
  (`KismetSystemLibrary.Delay` 0.2)
  (`self.UpdateDissolver`))

(fn `GetFarestActivatedCatalyseur`
  (returns (FarestActivatedCatalyseur :type "Actor Object Reference"))
  (locals (ActivatedCatalyseurList :type "Array of /Game/Blueprint/Nexus/BP_Catalyseur Object Reference"))
  (bind _returnvalue (`UsefullFunctions.SortActorsByDistanceToActor` (`local.ActivatedCatalyseurList`) self))
  (bind _result (`BlueprintSetLibrary.Set_ToArray` (`self.CatalyseurList`)))
  (for _array_element _result
    (if (`|EnumEquality` (`ActivableComponent.GetState` (`AbstractObjectif.ActivableComp` _array_element)) "CPF_Activated")
      (`KismetArrayLibrary.Array_Add` (`local.ActivatedCatalyseurList`) _array_element)))
  (return (`|GetArrayItem` _returnvalue (- (`KismetArrayLibrary.Array_Length` _returnvalue) 1))))

(fn `UpdateDissolver`
  (`/Game/Blueprint/FX/BP_Dissolver.DissolveTo` (`self.Dissolver`) (`self.GetDistanceTo` (`self.GetFarestActivatedCatalyseur`) self))
  (return))

(fn `UserConstructionScript`
  (`parent.UserConstructionScript`)
  (bind _outactors (`GameplayStatics.GetAllActorsOfClass` "/Game/Blueprint/FX/BP_Dissolver.BP_Dissolver_C"))
  (bind _output (`|GetArrayItem` _outactors))
  (`/Engine/EditorBlueprintResources/StandardMacros.IsValid` _output
    (:`Is Valid`
      (`self.K2_SetActorLocation` _output (`self.K2_GetActorLocation`) false false)
      (`/Game/Blueprint/FX/BP_Dissolver.UpdateShaderFX` _output))))