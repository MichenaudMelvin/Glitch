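; BP_Catalyseur is a catalyst object tied to the Nexus that switches its linked construction zones and spawners on and off.
; Activation requires specific Nexus and own states, then updates both lists; deactivation, also triggered by depleted health, sets them to the opposite state.
; BeginPlay falls back to the first BP_Nexus found if none is assigned.
; The construction script warns about and unlinks default-active zones, and corrects a disable wave set earlier than the enable wave.
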(event `self.ReceiveBeginPlay`
  (`parent.ReceiveBeginPlay`)
  (`/Engine/EditorBlueprintResources/StandardMacros.IsValid` (`self.Nexus`)
    (:`Is Not Valid`
      (`/Game/Blueprint/Helpers/FunctionLibrary/BP_UsefullFunctions.PrintWarn` (`KismetStringLibrary.Concat_StrStr` "nexus not assing to " (`KismetSystemLibrary.GetObjectName` self)))
      (bind _outactors (`GameplayStatics.GetAllActorsOfClass` "/Game/Blueprint/Nexus/BP_Nexus.BP_Nexus_C"))
      (set `self.Nexus` (`|GetArrayItem` _outactors)))))

(event `self.ActiveObject`
  (if (and (`|EnumEquality` (`/Game/Blueprint/Nexus/BP_AbstractObjectif.State` (`self.Nexus`)) "NewEnumerator0") (`|EnumEquality` (`self.State`) "NewEnumerator1"))
    (`parent.ActiveObject`)
    ;[1 0 0] Debug only
    (`/Game/Blueprint/Helpers/FunctionLibrary/BP_UsefullFunctions.Print` (`KismetStringLibrary.Concat_StrStr` (`KismetSystemLibrary.GetDisplayName` self) " activé"))
    (for _array_element (`self.ConstructionZoneList`)
      (`/Game/Blueprint/PlacableObjects/BP_ConstructionZone.UpdateState` _array_element "NewEnumerator0"))
    (for _array_element_2 (`self.SpawnerList`)
      (`/Game/Blueprint/AI/AISpawner/BP_Spawner.SetNewState` _array_element_2 "NewEnumerator0"))))

(event `self.Health.OnHealthNull`
  (`/Game/Blueprint/Nexus/BP_Nexus.DesactivateObject`))

(event `self.DesactivateObject`
  (`parent.DesactivateObject`)
  (for _array_element (`self.ConstructionZoneList`)
    (`/Game/Blueprint/PlacableObjects/BP_ConstructionZone.UpdateState` _array_element "NewEnumerator1"))
  (for _array_element_2 (`self.SpawnerList`)
    (`/Game/Blueprint/AI/AISpawner/BP_Spawner.SetNewState` _array_element_2 "NewEnumerator1")))

(fn `UserConstructionScript`
  (`parent.UserConstructionScript`)
  (for _array_element (`self.ConstructionZoneList`)
    (if (and (`|EnumEquality` (`/Game/Blueprint/PlacableObjects/BP_ConstructionZone.State` _array_element) "NewEnumerator0") (`KismetSystemLibrary.IsValid` _array_element))
      (`/Game/Blueprint/Helpers/FunctionLibrary/BP_UsefullFunctions.PrintWarn` (`KismetStringLibrary.Concat_StrStr` (`KismetSystemLibrary.GetDisplayName` _array_element) "est activé par défaut"))
      (`KismetArrayLibrary.Array_RemoveItem` (`self.ConstructionZoneList`) _array_element)))
  (if (< (`self.DisableAtWave`) (`self.EnableAtWave`))
    (set `self.DisableAtWave` (+ (`self.EnableAtWave`) 1))))