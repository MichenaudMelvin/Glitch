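; BP_AbstractObjectif is an objective actor, named as an abstract base, with health and an activation state.
; ActiveObject and DesactivateObject switch its State between two enum values.
; The Health component's damage event, along with BeginPlay, refreshes the ShowHealth text with current health.
; Tick rotates that text toward the player camera each frame so it works as a billboard.
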(event `self.ReceiveBeginPlay`
  (`self.UpdateHealth`))

(event `ActiveObject`
  (set `self.State` "NewEnumerator0"))

(event `DesactivateObject`
  (set `self.State` "NewEnumerator1"))

(event `self.Health.OnReciveDamages`
  (`self.UpdateHealth`))

(event `self.ReceiveTick`
  (params (DeltaSeconds :type "Float (single-precision)"))
  (`SceneComponent.K2_SetWorldRotation` (`self.ShowHealth`) (`KismetMathLibrary.FindLookAtRotation` (`SceneComponent.K2_GetComponentLocation` (`self.ShowHealth`)) (`self.K2_GetActorLocation` (`GameplayStatics.GetPlayerCameraManager` 0))) false false))

(fn `UpdateHealth`
  (`TextRenderComponent.K2_SetText` (`self.ShowHealth`) (`KismetTextLibrary.Conv_DoubleToText` (`HealthComponent.CurrentHealth` (`self.Health`)) "HalfToEven"))
  (return))

(fn `UserConstructionScript`)