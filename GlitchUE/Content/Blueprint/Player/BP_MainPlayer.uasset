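; Main player character Blueprint that implements dash and sprint, sneak, slide and ledge-cling movement.
; Movement events set speed and camera, rebind input through MainPlayerController and update ABP_Player state.
; A reversible timeline blends capsule height, mesh offset and speed for sneaking, while a looping timer decays slide velocity.
; Clinging attaches the player to an edge, moves the capsule, and limits sideways travel with finger/toe socket traces and edge bounds.
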(event `self.ReceiveBeginPlay`
  (`parent.ReceiveBeginPlay`)
  (set `self.MainPlayerController` (cast `MainPlayerController` (`self.GetController`) :!pure true))
  (set `self.NormalAcceleration` (`CharacterMovementComponent.MaxAcceleration` (`self.CharacterMovement`)))
  (set `self.OriginalMeshHeight` (.z (`SceneComponent.RelativeLocation` (`self.Mesh`))))
  (bind _output_get (set `self.SneakTime` (/ 1.0 (`self.SneakTime`))))
  (`TimelineComponent.SetPlayRate` (`self.SneakTimeline`) _output_get)
  (set `self.AnimBP` (cast `/Game/Animation/Player/ABP_Player` (`SkeletalMeshComponent.GetAnimInstance` (`self.Mesh`)) :!pure true)))

(event `self.Dash`
  ;[1 1 1] Sprint movements
  (`parent.Dash`)
  (`self.SetMovementMode` "Sprinting")
  (`MainPlayerController.BindSneak` (`self.MainPlayerController`))
  (if (`UsefulFunctions.IsCharacterMovingOnGround` self)
    ;;[0.35 1 0] Dash
    (set `CharacterMovementComponent.MaxAcceleration` (`self.DashAcceleration`) (`self.CharacterMovement`))
    (set `CharacterMovementComponent.MaxWalkSpeed` (`self.DashSpeed`) (`self.CharacterMovement`))
    (`self.CameraZoom` 1500.0)
    (`self.CameraFOV` 150.0)
    (`KismetSystemLibrary.Delay` (`self.DashDuration`))
    (switch `EPlayerMovementMode` (`self.GetMovementMode`)
      (:`Sprinting`
        (`self.Sprint`)))
    (else
      (`self.Sprint`))))

(event `Sprint`
  ;[1 1 1] Sprint movements
  (`self.CameraZoom` 400.0)
  (`self.CameraFOV` 100.0)
  ;;[0.35 1 0] Sprint
  (set `CharacterMovementComponent.MaxAcceleration` (`self.NormalAcceleration`) (`self.CharacterMovement`))
  (set `CharacterMovementComponent.MaxWalkSpeed` (`self.SprintSpeed`) (`self.CharacterMovement`)))

(event `self.SprintRelease`
  ;[1 1 1] Sprint movements
  (`parent.SprintRelease`)
  (if (`NavMovementComponent.IsFalling` (`self.CharacterMovement`))
    (set `self.ResetMovementOnLanded` true)
    (else
      (`self.ResetMovement`))))

(event `self.ResetMovement`
  (bind _mainplayercontroller (`self.MainPlayerController`))
  ;[1 1 1] ResetMovement
  (`parent.ResetMovement`)
  (switch `EPlayerMovementMode` (`self.GetMovementMode`)
    (:`Normal`
      _)
    (:`Sneaking`
      (`self.StandUP`))
    (:`Sprinting`
      _))
  (`self.SetMovementMode` "Normal")
  (set `CharacterMovementComponent.MaxAcceleration` (`self.NormalAcceleration`) (`self.CharacterMovement`))
  (set `CharacterMovementComponent.MaxWalkSpeed` (`self.NormalSpeed`) (`self.CharacterMovement`))
  (`self.CameraZoom` 300.0)
  (`self.CameraFOV` 90.0)
  (`/Game/Blueprint/Player/Controllers/BP_PC_MainPlayerController.BindSprint` _mainplayercontroller)
  (`MainPlayerController.BindSneak` _mainplayercontroller))

(event `self.OnLanded`
  (params (Hit :type "HitResult Structure (by ref)"))
  ;[1 1 1] ResetMovement
  (if (`self.ResetMovementOnLanded`)
    (set `self.ResetMovementOnLanded` false)
    (`self.ResetMovement`))
  (if (and (`|EnumEquality` (`self.GetMovementMode`) "Sneaking") (not (`UsefulFunctions.IsEventActionPressed` "Sneak" (`self.MainPlayerController`))))
    (`self.StandUP`)))

(event `ResetSneakPressed`
  ;[1 1 1] Sneak movements
  (`KismetSystemLibrary.K2_ClearAndInvalidateTimerHandle` (`self.SneakPressedTimer`))
  (goto _label :!via `Reset`))

(event `self.SneakPressed`
  ;[1 1 1] Sneak movements
  (`KismetSystemLibrary.K2_ClearAndInvalidateTimerHandle` (`self.StandUPTimer`))
  (bind _returnvalue (`KismetSystemLibrary.K2_SetTimerDelegate` (`|CreateDelegate` :!event `Sneak`) 0.001 true))
  (set `self.SneakPressedTimer` _returnvalue))

(event `self.FinishGlitchDash`
  (bind _currentedge (`self.CurrentEdge`))
  (`parent.FinishGlitchDash`)
  (`/Engine/EditorBlueprintResources/StandardMacros.IsValid` _currentedge
    (:`Is Valid`
      (`self.AttachPlayerToEdge` _currentedge))))

(event `Sneak`
  (bind _mainplayercontroller (`self.MainPlayerController`))
  (bind _originalmeshheight (`self.OriginalMeshHeight`))
  ;[1 1 1] Sneak movements
  (if (`|EnumInequality` (`self.GetMovementMode`) "Sneaking")
    (`|ExecutionSequence`
      (:`then_0`
        (`/Engine/EditorBlueprintResources/StandardMacros.DoOnce` false :!label _label
          (:`Completed`
            (`self.SelectTargetLerpSpeed` (`self.GetMovementMode`))
            (`self.SetMovementMode` "Sneaking")
            (`self.CameraZoom` 200.0)
            (`/Game/Blueprint/Player/Controllers/BP_PC_MainPlayerController.BindSprint` (`self.MainPlayerController`)))))
      (:`then_1`
        (bind (_direction _sneakvalue) (`Timeline|SneakTimeline` :!label _label_2)
          (:`Update`
            (if (not (`self.LerpSneakSpeed`))
              (set `CharacterMovementComponent.MaxWalkSpeed` (`KismetMathLibrary.Lerp` (`self.TargetLerpSpeed`) (`self.SneakSpeed`) _sneakvalue) (`self.CharacterMovement`)))
            (bind _returnvalue (`KismetMathLibrary.Lerp` (`self.HalfHeight`) (`self.SneakHalfHeight`) _sneakvalue))
            ;;[0.35 1 0] Lerp la vitesse, la taille de la capsule et la position relative du mesh
            (`CapsuleComponent.SetCapsuleHalfHeight` (`self.CapsuleComponent`) _returnvalue true)
            (set `/Game/Animation/Player/ABP_Player.CapsuleHalfHeight` _returnvalue (`self.AnimBP`))
            (`SceneComponent.K2_SetRelativeLocation` (`self.Mesh`) (`KismetMathLibrary.MakeVector` 0.0 0.0 (`KismetMathLibrary.Lerp` _originalmeshheight (/ _originalmeshheight 2.0) _sneakvalue)) false false))
          (:`Finished`
            (if (not (`/Game/Animation/Player/ABP_Player.IsSliding` (`self.AnimBP`)))
              (switch `ETimelineDirection` _direction
                (:`Forward`
                  (`self.SetMovementMode` "Sneaking")
                  (`self.ResetSneakPressed`)
                  (`/Game/Blueprint/Player/Controllers/BP_PC_MainPlayerController.BindSneak` _mainplayercontroller)
                  (`/Game/Blueprint/Player/Controllers/BP_PC_MainPlayerController.BindSprint` _mainplayercontroller))
                (:`Backward`
                  (`self.ResetMovement`))))))))))

(event `self.SneakReleased`
  ;[1 1 1] Sneak movements
  (`self.ResetSneakPressed`)
  (bind _returnvalue (`KismetSystemLibrary.K2_SetTimerDelegate` (`|CreateDelegate` :!event `StandUP`) 0.001 true))
  (set `self.StandUPTimer` _returnvalue))

(event `StopSneakTimeline`
  ;[1 1 1] Sneak movements
  (goto _label_2 :!via `Stop`))

(event `self.DetachFromEdge`
  ;[1 1 1] Cling
  (`parent.DetachFromEdge`)
  (`self.K2_DetachFromActor` "KeepWorld" "KeepWorld" "KeepWorld")
  (set `self.CurrentEdge` null)
  (set `/Game/Animation/Player/ABP_Player.IsClimbing` false (`self.AnimBP`))
  (switch `EDirection` (`/Game/Animation/Player/ABP_Player.ClimbDirection` (`self.AnimBP`))
    (:`Left`
      _)
    (:`Right`
      _))
  (`self.StopHorizontalClingMovement`))

(event `StandUP`
  ;[1 1 1] Sneak movements
  (if (`self.CanStandUP`)
    (`KismetSystemLibrary.K2_ClearAndInvalidateTimerHandle` (`self.StandUPTimer`))
    (goto _label_2 :!via `Reverse`)))

(event `StopHorizontalClingMovement`
  (bind _slideanimation (`self.SlideAnimation`))
  (bind _climbdirection (`/Game/Animation/Player/ABP_Player.ClimbDirection` (`self.AnimBP`)))
  ;[1 1 1] Cling
  (goto _label_3 :!via `Stop`))

(event `self.HorizontalCling`
  (params (Direction :type "EDirection Enum" :default "Up"))
  (bind (_canmove _distance) (`self.CheckCanMoveAtTargetDirection` Direction))
  (bind _slideanimation (`self.SlideAnimation`))
  (bind _climbdirection (`/Game/Animation/Player/ABP_Player.ClimbDirection` (`self.AnimBP`)))
  (bind _returnvalue (/ 1.0 (`UsefulFunctions.GetAnimLength` (select `EDirection` Direction :`Up` _slideanimation :`Down` _slideanimation :`Left` (`self.ClingLeftAnimation`) :`Right` (`self.ClingRightAnimation`) :`None` _slideanimation))))
  ;[1 1 1] Cling
  (if _canmove
    (set `/Game/Animation/Player/ABP_Player.ClimbDirection` Direction (`self.AnimBP`))
    (`|ExecutionSequence`
      (:`then_0`
        (`KismetSystemLibrary.MoveComponentTo` (`self.CapsuleComponent`) (`UsefulFunctions.AddToVector` (`SceneComponent.RelativeLocation` (`self.CapsuleComponent`)) _distance) (`SceneComponent.RelativeRotation` (`self.CapsuleComponent`)) false false _returnvalue :!label _label_3)
        (if (or (`|EnumEquality` _climbdirection "Left") (`|EnumEquality` _climbdirection "Right"))
          (set `MovementComponent.Velocity` (0.0 0.0 0.0) (`self.CharacterMovement`))
          (set `/Game/Animation/Player/ABP_Player.ClimbDirection` "None" (`self.AnimBP`) :!label _label_4)))
      (:`then_1`
        (`KismetSystemLibrary.RetriggerableDelay` (/ _returnvalue 2.0))
        (goto _label_4)))))

(event `self.SneakToSprint`
  (bind _mainplayercontroller (`self.MainPlayerController`))
  ;[1 1 1] Sneak movements
  (`parent.SneakToSprint`)
  (if (`self.CanStandUP`)
    (`self.StopSneakTimeline`)
    (set `self.LerpSneakSpeed` true)
    (`self.StandUP`)
    (`self.Dash`)
    (`KismetSystemLibrary.Delay` (`UsefulFunctions.GetTimelineDuration` (`self.SneakTimeline`)))
    (set `self.LerpSneakSpeed` false)
    (`self.SetMovementMode` "Sprinting")
    (`/Game/Blueprint/Player/Controllers/BP_PC_MainPlayerController.BindSneak` _mainplayercontroller)
    (`/Game/Blueprint/Player/Controllers/BP_PC_MainPlayerController.BindSprint` _mainplayercontroller)))

(event `self.SprintToSneak`
  (bind _mainplayercontroller (`self.MainPlayerController`))
  (bind _charactermovement (`self.CharacterMovement`))
  ;[1 1 1] Sneak movements
  (if (`UsefulFunctions.IsCharacterMovingOnGround` self)
    (`self.StopSneakTimeline`)
    (set `self.SlideVelocity` (`MovementComponent.Velocity` (`self.CharacterMovement`)))
    (set `self.SlideTimer` 0.0)
    (set `CharacterMovementComponent.GroundFriction` 0.0 _charactermovement)
    (set `CharacterMovementComponent.BrakingDecelerationWalking` 1024.0 _charactermovement)
    (bind _returnvalue (`KismetSystemLibrary.K2_SetTimerDelegate` (`|CreateDelegate` :!event `Slide`) 0.1 true))
    (set `self.SlideTimerHandle` _returnvalue)
    (`TimelineComponent.SetPlayRate` (`self.SneakTimeline`) (/ 1.0 (`UsefulFunctions.GetAnimLength` (`self.SlideAnimation`))))
    (set `/Game/Animation/Player/ABP_Player.IsSliding` true (`self.AnimBP`))
    (`MainPlayerController.UnbindAll` _mainplayercontroller false)
    (`MainPlayerController.BindInteraction` _mainplayercontroller)
    (add `MainPlayerController.OnSneakReleased` _mainplayercontroller (`|CreateDelegate` :!event `ReleasedSlide`))
    (`self.LookAtTarget` (`self.K2_GetActorRotation`) (`|CreateDelegate` (`self.MainPlayerController`) :!event `BindCamera`) 0.5)
    (`self.Sneak`)
    (clear `MainPlayerController.OnSprintPressed` (`self.MainPlayerController`))
    (else
      (`self.ResetMovement`)
      (`self.Sneak`))))

(event `self.ClingUp`
  (bind _animbp (`self.AnimBP`))
  ;[1 1 1] Cling
  (`MainPlayerController.UnbindAll` (`self.MainPlayerController`) false)
  (set `/Game/Animation/Player/ABP_Player.ClimbDirection` "Up" _animbp)
  (`self.StopHorizontalClingMovement`)
  (set `/Game/Animation/Player/ABP_Player.IsClimbing` false _animbp)
  (`KismetSystemLibrary.MoveComponentTo` (`self.CapsuleComponent`) (`/Game/Blueprint/Rebords/BP_Edge.GetUpperHeightLocation` (`self.CurrentEdge`)) (`SceneComponent.RelativeRotation` (`self.CapsuleComponent`)) false false (`self.GetClimbUpAnimDuration`))
  (set `/Game/Animation/Player/ABP_Player.ClimbDirection` "None" (`self.AnimBP`))
  (`KismetSystemLibrary.MoveComponentTo` (`self.CapsuleComponent`) (`/Game/Blueprint/Rebords/BP_Edge.GetUpperLocation` (`self.CurrentEdge`)) (`SceneComponent.RelativeRotation` (`self.CapsuleComponent`)) false false (`self.GetClimbUpAnimDuration`))
  (`self.DetachFromEdge`) ; Par sécurité
)

(event `Slide`
  ;[1 1 1] Sneak movements
  (bind _output_get (set `self.SlideTimer` (+ (`self.SlideTimer`) 0.1)))
  (bind _output_get_2 (set `self.SlideNormalizedTimer` (`KismetMathLibrary.NormalizeToRange` _output_get 0.0 (`self.SlideDuration`))))
  (bind _output_get_3 (set `MovementComponent.Velocity` (`KismetMathLibrary.VLerp` (`self.SlideVelocity`) (0.0 0.0 0.0) _output_get_2) (`self.CharacterMovement`)))
  (if (or (== _output_get_3 (0.0 0.0 0.0) :`ErrorTolerance` 1.0) (`KismetMathLibrary.NearlyEqual_FloatFloat` (.x (`SceneComponent.GetComponentVelocity` (`self.CapsuleComponent`))) 0.0 1.0) (`KismetMathLibrary.NearlyEqual_FloatFloat` (.y (`SceneComponent.GetComponentVelocity` (`self.CapsuleComponent`))) 0.0 1.0) (not (`UsefulFunctions.IsCharacterMovingOnGround` self)))
    (`self.ReleasedSlide`)))

(event `ReleasedSlide`
  (bind _charactermovement (`self.CharacterMovement`))
  ;[1 1 1] Sneak movements
  (`KismetSystemLibrary.K2_ClearAndInvalidateTimerHandle` (`self.SlideTimerHandle`))
  (`self.StopLookAtTimeline`)
  (`MainPlayerController.BindNormalMode` (`self.MainPlayerController`))
  (set `CharacterMovementComponent.GroundFriction` (`self.OriginalGroundFriction`) _charactermovement)
  (set `CharacterMovementComponent.BrakingDecelerationWalking` (`self.OriginalBrakingDecelerationWalking`) _charactermovement)
  (`TimelineComponent.SetPlayRate` (`self.SneakTimeline`) (`self.SneakTime`))
  (if (and (< (`self.SlideNormalizedTimer`) 1.0) (`self.CanStandUP`))
    (`KismetSystemLibrary.Delay` (`UsefulFunctions.GetTimelineDuration` (`self.SneakTimeline`)))
    (`self.SetMovementMode` "Sprinting")
    (set `self.TargetLerpSpeed` (`self.NormalSpeed`))
    (`self.StandUP`)
    (`self.ResetMovement`)
    (set `/Game/Animation/Player/ABP_Player.IsSliding` false (`self.AnimBP`))
    (else
      (`self.SetMovementMode` "Normal")
      (`self.ResetSneakPressed`)
      (`self.Sneak`)
      (set `/Game/Animation/Player/ABP_Player.IsSliding` false (`self.AnimBP`))
      (if (not (`UsefulFunctions.IsEventActionPressed` "Sneak" (`self.MainPlayerController`)))
        (bind _returnvalue (`KismetSystemLibrary.K2_SetTimerDelegate` (`|CreateDelegate` :!event `StandUP`) 0.001 true))
        (set `self.StandUPTimer` _returnvalue)))))

(fn `AttachPlayerToEdge`
  (params (Edge :type "/Game/Blueprint/Rebords/BP_Edge Object Reference") (CollideWithLowerEdge :type Boolean :default true))
  (bind _mainplayercontroller (`self.MainPlayerController`))
  (bind _animbp (`self.AnimBP`))
  (bind _currentedge (`self.CurrentEdge`))
  (set `self.CurrentEdge` Edge)
  (set `/Game/Animation/Player/ABP_Player.IsClimbing` true _animbp)
  (set `/Game/Animation/Player/ABP_Player.ClimbDirection` (select `bool` CollideWithLowerEdge :`false` "Up" :!type "EDirection Enum") _animbp)
  (set `CharacterMovementComponent.GravityScale` 0.0 (`self.CharacterMovement`))
  (set `MovementComponent.Velocity` (0.0 0.0 0.0) (`self.CharacterMovement`))
  (`self.StopJumping`)
  (`self.K2_AttachToActor` (`self.CurrentEdge`) "None" "KeepWorld" "KeepWorld" "KeepWorld")
  (`self.K2_SetActorRotation` (`/Game/Blueprint/Rebords/BP_Edge.GetEdgeRotation` (`self.CurrentEdge`)))
  (`self.K2_SetActorRelativeLocation` (`KismetMathLibrary.SelectVector` (`/Game/Blueprint/Rebords/BP_Edge.GetLowerLocation` _currentedge) (`/Game/Blueprint/Rebords/BP_Edge.GetUpperLocation` _currentedge) (`local.CollideWithLowerEdge`)))
  (`self.CameraAimReverse`)
  (`MainPlayerController.UnbindGlitch` _mainplayercontroller)
  (`MainPlayerController.UnbindMouseScroll` _mainplayercontroller)
  (`MainPlayerController.BindClingMovement` _mainplayercontroller)
  (return))

(fn `CheckCanMoveAtTargetDirection`
  (params (ClingDirection :type "EDirection Enum" :default "Up"))
  (returns (CanMove :type Boolean) (Distance :type "Float (double-precision)"))
  (locals (DirectionName :type String) (FingersLineTrace :type Boolean :default false) (ToesLineTrace :type Boolean :default false) (FingersLineTraceDistance :type "Float (double-precision)" :default 0.0) (ToesLineTraceDistance :type "Float (double-precision)" :default 0.0))
  (bind _returnvalue (`SceneComponent.GetSocketLocation` (`self.Mesh`) (`KismetStringLibrary.Conv_StringToName` (`KismetStringLibrary.Concat_StrStr` (`local.DirectionName`) "Toes"))))
  (bind _returnvalue_2 (`SceneComponent.GetSocketLocation` (`self.Mesh`) (`KismetStringLibrary.Conv_StringToName` (`KismetStringLibrary.Concat_StrStr` (`local.DirectionName`) "Fingers"))))
  (bind _returnvalue_3 (select `bool` (or (`local.FingersLineTrace`) (`local.ToesLineTrace`)) :`false` (`self.GetHorizontalDistance` (`self.ClingHorizontalDistance`) (`local.ClingDirection`)) :`true` (`self.GetHorizontalDistance` (- (`KismetMathLibrary.FMin` (`KismetMathLibrary.SelectFloat` (`local.FingersLineTraceDistance`) (`self.ClingHorizontalDistance`) (`local.FingersLineTrace`)) (`KismetMathLibrary.SelectFloat` (`local.ToesLineTraceDistance`) (`self.ClingHorizontalDistance`) (`local.ToesLineTrace`))) (`self.GetHorizontalTolerance`)) (`local.ClingDirection`))))
  (`/Engine/EditorBlueprintResources/StandardMacros.IsValid` (`self.CurrentEdge`)
    (:`Is Valid`
      (set `local.DirectionName` (select `EDirection` ClingDirection :`Left` "Left" :`Right` "Right"))
      (bind (_outhit _returnvalue_4) (`KismetSystemLibrary.LineTraceSingle` :`Start` _returnvalue_2 :`End` (+ _returnvalue_2 (* (* (`self.GetActorRightVector`) -1) (`self.GetHorizontalDistance` (`self.ClingHorizontalDistance`) (`local.ClingDirection`)))) :`TraceChannel` "TraceTypeQuery1" :`TraceColor` (struct :`G` 0.009524 :`B` 1.0 :`A` 1.0) :`DrawTime` 2.0))
      (set `local.FingersLineTrace` _returnvalue_4)
      (set `local.FingersLineTraceDistance` (`.Distance` (`GameplayStatics.BreakHitResult` _outhit)))
      (if (`local.FingersLineTrace`)
        (if (`self.CheckHorizontalLineTraceDistance` (`local.FingersLineTraceDistance`))
          (return false 0.0)
          (else
            _)))
      (bind (_outhit_2 _returnvalue_5) (`KismetSystemLibrary.LineTraceSingle` :`Start` _returnvalue :`End` (+ _returnvalue (* (* (`self.GetActorRightVector`) -1) (`self.GetHorizontalDistance` (`self.ClingHorizontalDistance`) (`local.ClingDirection`)))) :`TraceChannel` "TraceTypeQuery1" :`TraceColor` (struct :`R` 1.0 :`B` 0.004663 :`A` 1.0) :`DrawTime` 2.0))
      (set `local.ToesLineTrace` _returnvalue_5)
      (set `local.ToesLineTraceDistance` (`.Distance` (`GameplayStatics.BreakHitResult` _outhit_2)))
      (if (`local.ToesLineTrace`)
        (if (`self.CheckHorizontalLineTraceDistance` (`local.ToesLineTraceDistance`))
          (return false 0.0)
          (else
            _)))
      (return true (`KismetMathLibrary.SelectFloat` _returnvalue_3 (`self.GetOutsideEdgeValue` (`local.ClingDirection`)) (`/Game/Blueprint/Rebords/BP_Edge.Is Value Inside the Edge` (`self.CurrentEdge`) _returnvalue_3))))
    (:`Is Not Valid`
      (return false 0.0))))

(fn `CheckHorizontalLineTraceDistance`
  (params (LineTraceDistance :type "Float (double-precision)"))
  (returns (ReturnValue :type Boolean))
  (return (< LineTraceDistance (`self.GetHorizontalTolerance`))))

(fn `GetClimbUpAnimDuration`
  (returns (ReturnValue :type "Float (double-precision)"))
  (return (/ (/ 1.0 (`UsefulFunctions.GetAnimLength` (`self.ClingUpAnimation`))) 2.0)))

(fn `GetHorizontalDistance`
  (params (DistanceModifier :type "Float (double-precision)") (Direction :type "EDirection Enum" :default "Up"))
  (returns (HorizontalDistance :type "Float (double-precision)"))
  (return (select `EDirection` (`local.Direction`) :`Left` DistanceModifier :`Right` (* -1 DistanceModifier))))

(fn `GetHorizontalTolerance`
  (returns (HorizontalTolerance :type "Float (double-precision)"))
  (return (+ (`self.HorizontalTolerance`) (`CapsuleComponent.CapsuleRadius` (`self.CapsuleComponent`)))))

(fn `GetOutsideEdgeValue`
  (params (ClingDirection :type "EDirection Enum" :default "Up"))
  (returns (HorizontalDistance :type "Float (double-precision)"))
  (return (`self.GetHorizontalDistance` (- (- (`/Game/Blueprint/Rebords/BP_Edge.BoxLength` (`self.CurrentEdge`)) (`KismetMathLibrary.Abs` (.x (`SceneComponent.RelativeLocation` (`self.CapsuleComponent`))))) (`self.GetHorizontalTolerance`)) (`local.ClingDirection`))))

(fn `SelectTargetLerpSpeed`
  (params (TargetMovementMode :type "EPlayerMovementMode Enum" :default "Normal"))
  (set `self.TargetLerpSpeed` (select `EPlayerMovementMode` (`local.TargetMovementMode`) :`Normal` (`self.NormalSpeed`) :`Sneaking` (`self.SneakSpeed`) :`Sprinting` (`self.SprintSpeed`)))
  (return))

(fn `UserConstructionScript`)