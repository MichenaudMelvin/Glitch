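; Game mode for a transition level that shows narrative chat messages between game sequences and selects the next level to load.
; After a short delay on BeginPlay, it switches on OptionsString to push that transition's lines to TchatWidget and set LevelToLoad.
; FinishRead opens LevelToLoad; unmatched or empty options call it immediately, while matched cases leave it to be triggered from outside this graph.
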(event `self.ReceiveBeginPlay`
  (`parent.ReceiveBeginPlay`)
  (`KismetSystemLibrary.Delay` 0.2)
  (switch `string` (`self.OptionsString`)
    (:`Default`
      (`self.FinishRead` :!label _label))
    (:`?FromMainMenuToMovingSequence`
      (`Tchat.AddMultipleTchatLines` (`self.TchatWidget`) (`self.MainMenuToMovingMessages`))
      (set `self.LevelToLoad` "/Game/Maps/Playable-Level/LVL-Moving-Sequence.LVL-Moving-Sequence"))
    (:`?FromMovingToStealth`
      (`Tchat.AddMultipleTchatLines` (`self.TchatWidget`) (`self.MovingFromStealthMessages`))
      (set `self.LevelToLoad` "/Game/Maps/Playable-Level/LVL-Infiltration.LVL-Infiltration"))
    (:`?FromStealthToTowerDefense`
      (`Tchat.AddTchatLine` (`self.TchatWidget`) "Console" "Congratulation, you came back. Now  we can continue the test. Free the nexus." (struct :`R` 0.938433 :`G` 1.0 :`A` 1.0))
      (set `self.LevelToLoad` "/Game/Maps/Playable-Level/LVL-TWD.LVL-TWD"))
    (:`?FromTowerDefenseToLevelOne`
      (`Tchat.AddMultipleTchatLines` (`self.TchatWidget`) (`self.TowerDefenseToLevelOneMessages`))
      (set `self.LevelToLoad` "/Game/Maps/Playable-Level/LVL-1.LVL-1"))
    (:`None`
      (goto _label))
    (:`?`
      (goto _label))))

(event `FinishRead`
  (`GameplayStatics.OpenLevelBySoftObjectPtr` (`self.LevelToLoad`)))

(fn `UserConstructionScript`)