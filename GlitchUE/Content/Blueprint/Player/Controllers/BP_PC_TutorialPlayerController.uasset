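; Player controller for the tutorial that captures player input for movement, camera, jumping, interaction, glitch use, object placement, quick save/load and pause.
; Each input action or axis is relayed through a matching event dispatcher call, leaving gameplay responses to whatever binds to them.
; The chat input is the exception, using a FlipFlop to open and close the Tchat object directly.
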(event `InputAxis|MoveForward`
  (params (AxisValue :type "Float (single-precision)"))
  ;[1 1 1] Basic movement and camera
  (`self.OnMoveForward` AxisValue))

(event `InputAxis|MoveRight`
  (params (AxisValue :type "Float (single-precision)"))
  ;[1 1 1] Basic movement and camera
  (`self.OnMoveRight` AxisValue))

(event `InputAction|Interact`
  (params (Key :type "Key Structure"))
  ;[1 1 1] Specific actions
  (:`Pressed`
    (`self.OnInteractPlayer`)))

(event `InputAction|Jump`
  (params (Key :type "Key Structure"))
  ;[1 1 1] Specific actions
  (:`Pressed`
    (`self.OnJumpPressed`))
  (:`Released`
    (`self.OnJumpReleased`)))

(event `InputAction|MouseScroll`
  (params (Key :type "Key Structure"))
  ;[1 1 1] Specific actions
  (:`Pressed`
    (`self.OnMouseScroll` (`self.GetInputAxisKeyValue` Key))))

(event `InputAction|OpenTchat`
  (params (Key :type "Key Structure"))
  (bind _tchat (`self.Tchat`))
  ;[1 1 1] Specific actions
  (:`Pressed`
    (`/Engine/EditorBlueprintResources/StandardMacros.FlipFlop`
      (:`A`
        (`Tchat.OpenTchat` _tchat))
      (:`B`
        (`Tchat.CloseTchat` _tchat)))))

(event `InputAxis|Turn`
  (params (AxisValue :type "Float (single-precision)"))
  ;[1 1 1] Basic movement and camera
  (`self.OnTurn` AxisValue))

(event `InputAxis|LookUp`
  (params (AxisValue :type "Float (single-precision)"))
  ;[1 1 1] Basic movement and camera
  (`self.OnLookUp` AxisValue))

(event `InputAction|Sprint`
  (params (Key :type "Key Structure"))
  ;[1 1 1] Specific actions
  (:`Pressed`
    (`self.OnSprintPressed`))
  (:`Released`
    (`self.OnSprintReleased`)))

(event `InputAction|Sneak`
  (params (Key :type "Key Structure"))
  ;[1 1 1] Specific actions
  (:`Pressed`
    (`self.OnSneakPressed`))
  (:`Released`
    (`self.OnSneakReleased`)))

(event `Key|AnyKey` :paused true
  (params (Key :type "Key Structure"))
  ;[1 1 1] Specific actions
  (:`Pressed`
    (`AbstractPlayerController.OnAnyKey` Key)))

(event `InputAxis|TurnRate`
  (params (AxisValue :type "Float (single-precision)"))
  ;[1 1 1] Basic movement and camera
  (`self.OnTurnRate` AxisValue))

(event `InputAxis|LookUpRate`
  (params (AxisValue :type "Float (single-precision)"))
  ;[1 1 1] Basic movement and camera
  (`self.OnLookUpRate` AxisValue))

(event `InputAction|PlaceObject`
  (params (Key :type "Key Structure"))
  ;[1 1 1] Specific actions
  (:`Pressed`
    (`self.OnPlaceObject`)))

(event `InputAction|UseGlitch`
  (params (Key :type "Key Structure"))
  ;[1 1 1] Specific actions
  (:`Pressed`
    (`self.OnUseGlitchPressed`))
  (:`Released`
    (`self.OnUseGlitchReleased`)))

(event `InputAction|FastSave`
  (params (Key :type "Key Structure"))
  ;[1 1 1] Specific actions
  (:`Pressed`
    (`self.OnFastSave`)))

(event `InputAction|FastLoad`
  (params (Key :type "Key Structure"))
  ;[1 1 1] Specific actions
  (:`Pressed`
    (`self.OnFastLoad`)))

(event `InputAction|Pause` :paused true
  (params (Key :type "Key Structure"))
  ;[1 1 1] Pause game
  (:`Pressed`
    (`self.OnPause`)))

(fn `UserConstructionScript`)