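; Player controller for the transition game mode that hooks into a chat ("Tchat") widget and signals when reading is finished.
; After a short delay on BeginPlay, it binds to the widget's message-list-finished and extend-start events.
; The OpenTchat input fires the CloseTchat dispatcher, which a separate Bind event subscribes to.
; When OnCloseTchat receives a false Forward flag, it calls FinishRead on BP_TransitionGamemode.
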(event `self.ReceiveBeginPlay`
  (`parent.ReceiveBeginPlay`)
  (`KismetSystemLibrary.Delay` 0.2)
  (add `Tchat.OnFinishWritingMessageList` (`self.TchatWidget`) (`|CreateDelegate` :!event `Bind`))
  (add `Tchat.OnTchatExtendStart` (`self.TchatWidget`) (`|CreateDelegate` :!event `OnCloseTchat`)))

(event `InputAction|OpenTchat`
  (params (Key :type "Key Structure"))
  (:`Pressed`
    (`self.CloseTchat`)))

(event `Bind`
  (add `self.CloseTchat` (`|CreateDelegate` (`self.TchatWidget`) :!event `CloseTchat`)))

(event `OnCloseTchat`
  (params (Forward :type Boolean))
  (if (not Forward)
    (`/Game/Blueprint/Player/Gamemodes/BP_TransitionGamemode.FinishRead` (cast `/Game/Blueprint/Player/Gamemodes/BP_TransitionGamemode` (`self.Gamemode`) :!pure true))))

(fn `UserConstructionScript`)