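; Main player controller that routes input to the player's movement, glitch and object-building actions and owns the game's UI widgets.
; Input events only fire dispatchers; Bind/Unbind functions, some overriding parent versions, rewire listeners per context, though many graph copies are disconnected.
; Construction binds a looping preview timer, placement and 90-degree rotation.
; The object wheel slows time while open, and a quick release returns to Normal mode.
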(event `self.ReceiveBeginPlay`
  (`parent.ReceiveBeginPlay`)
  (set `self.MainPlayer` (cast `/Game/Blueprint/Player/BP_MainPlayer` (`GameplayStatics.GetPlayerCharacter` 0) :!pure true))
  (`|ExecutionSequence`
    (:`then_0`
      (bind _returnvalue (`|CreateWidget` "/Game/Blueprint/PlacableObjects/UI/WBP_PlacableObjectsWheelSelection.WBP_PlacableObjectsWheelSelection_C"))
      (bind _output_get (set `self.PlacableObjectWheel` _returnvalue))
      (`/Game/Blueprint/PlacableObjects/UI/WBP_PlacableObjectsWheelSelection.CreateWheelButton` _output_get (`self.PlacableObjectList`)))
    (:`then_1`
      (bind _returnvalue_2 (`|CreateWidget` "/Game/Blueprint/Player/UI/WBP_PauseMenu.WBP_PauseMenu_C"))
      (set `self.PauseWidget` _returnvalue_2))
    (:`then_2`
      (bind _returnvalue_3 (`|CreateWidget` "/Game/Blueprint/Player/UI/WBP_Sight.WBP_Sight_C"))
      (set `self.SightWidget` _returnvalue_3))
    (:`then_3`
      (bind _returnvalue_4 (`|CreateWidget` "/Game/Blueprint/Player/UI/WBP_DisplayStats.WBP_DisplayStats_C"))
      (bind _output_get_2 (set `self.DisplayStats` _returnvalue_4))
      (`UserWidget.AddToViewport` _output_get_2 0))
    (:`then_4`
      (bind _returnvalue_5 (`|CreateWidget` "/Game/Blueprint/Nexus/UI/WBP_WaveManaging.WBP_WaveManaging_C"))
      (set `self.WaveManagerUI` _returnvalue_5))))

(event `InputAxis|MoveForward`
  (params (AxisValue :type "Float (single-precision)"))
  ;[1 1 1] Basic movement and camera
  (`self.OnMoveForward` AxisValue))

(event `InputAxis|MoveRight`
  (params (AxisValue :type "Float (single-precision)"))
  ;[1 1 1] Basic movement and camera
  (`self.OnMoveRight` AxisValue))

(event `InputAction|Interact`
  (params (Key :type "Key Structure"))
  ;[1 1 1] Specific actions
  (:`Pressed`
    (`self.OnInteractPlayer`)))

(event `InputAction|Jump`
  (params (Key :type "Key Structure"))
  ;[1 1 1] Specific actions
  (:`Pressed`
    (`self.OnJumpPressed`))
  (:`Released`
    (`self.OnJumpReleased`)))

(event `InputAction|RotateObjects`
  (params (Key :type "Key Structure"))
  ;[1 1 1] Specific actions
  (:`Pressed`
    (`self.OnRotateObjects` (`self.GetInputAxisKeyValue` Key))))

(event `InputAxis|Turn`
  (params (AxisValue :type "Float (single-precision)"))
  ;[1 1 1] Basic movement and camera
  (`self.OnTurn` AxisValue))

(event `InputAxis|LookUp`
  (params (AxisValue :type "Float (single-precision)"))
  ;[1 1 1] Basic movement and camera
  (`self.OnLookUp` AxisValue))

(event `InputAction|Sprint`
  (params (Key :type "Key Structure"))
  ;[1 1 1] Specific actions
  (:`Pressed`
    (`self.OnSprint`)))

(event `InputAction|Sneak`
  (params (Key :type "Key Structure"))
  ;[1 1 1] Specific actions
  (:`Pressed`
    (`self.OnSneakPressed`))
  (:`Released`
    (`self.OnSneakReleased`)))

(event `InputAction|RotateObjectsLeft`
  (params (Key :type "Key Structure"))
  ;[1 1 1] Specific actions
  (:`Pressed`
    (`self.OnRotateObjectsLeft` -1.0)))

(event `InputAction|OpenSelectionWheel`
  (params (Key :type "Key Structure"))
  ;[1 1 1] Specific actions
  (:`Pressed`
    (`self.OnOpenSelectionWheelPressed`))
  (:`Released`
    (`self.OnOpenSelectionWheelReleased`)))

(event `InputAxis|TurnRate`
  (params (AxisValue :type "Float (single-precision)"))
  ;[1 1 1] Basic movement and camera
  (`self.OnTurnRate` AxisValue))

(event `InputAxis|LookUpRate`
  (params (AxisValue :type "Float (single-precision)"))
  ;[1 1 1] Basic movement and camera
  (`self.OnLookUpRate` AxisValue))

(event `InputAction|PlaceObject`
  (params (Key :type "Key Structure"))
  ;[1 1 1] Specific actions
  (:`Pressed`
    (`self.OnPlaceObject`)))

(event `InputAction|UseGlitch`
  (params (Key :type "Key Structure"))
  ;[1 1 1] Specific actions
  (:`Pressed`
    (`self.OnUseGlitchPressed`))
  (:`Released`
    (`self.OnUseGlitchReleased`)))

(event `InputAction|RotateObjectsRight`
  (params (Key :type "Key Structure"))
  ;[1 1 1] Specific actions
  (:`Pressed`
    (`self.OnRotateObjectsRight` 1.0)))

(event `InputAction|Pause` :paused true
  (params (Key :type "Key Structure"))
  ;[1 1 1] Pause game
  (:`Pressed`
    (`self.OnPause`)))

(event `PauseGame`
  (bind _pausewidget (`self.PauseWidget`))
  ;[1 1 1] Pause game
  (`GameplayStatics.SetGamePaused` (not (`GameplayStatics.IsGamePaused`)))
  (set `self.bShowMouseCursor` (not (`self.bShowMouseCursor`)))
  (if (`Widget.IsInViewport` _pausewidget)
    (`Widget.RemoveFromParent` _pausewidget)
    (else
      (`UserWidget.AddToViewport` _pausewidget 0))))

(event `self.BindSprint`
  (`parent.BindSprint`)
  (switch `EPlayerMovementMode` (`MainPlayer.GetMovementMode` (`self.MainPlayer`))
    (:`Normal`
      (add `self.OnSprint` (`|CreateDelegate` (`self.MainPlayer`) :!event `Dash`)))
    (:`Sneaking`
      (add `self.OnSprint` (`|CreateDelegate` (`self.MainPlayer`) :!event `SneakToSprint`)))
    (:`Sprinting`
      (add `self.OnSprint` (`|CreateDelegate` (`self.MainPlayer`) :!event `Dash`)))))

(event `self.BindOpenSelectionWheel`
  (`self.UnbindOpenSelectionWheel`)
  (add `self.OnOpenSelectionWheelPressed` (`|CreateDelegate` :!event `Open`))
  (add `self.OnOpenSelectionWheelReleased` (`|CreateDelegate` :!event `CloseWheel`)))

(event `self.BindConstruction`
  (bind _returnvalue (`KismetSystemLibrary.K2_SetTimerDelegate` (`|CreateDelegate` (`self.MainPlayer`) :!event `PreviewActor`) 0.1 true))
  (set `self.PreviewObjectTimerHandle` _returnvalue)
  (add `self.OnPlaceObject` (`|CreateDelegate` (`self.MainPlayer`) :!event `PlaceActor`))
  (`self.BindRotateObjects`))

(event `self.UnbindOpenSelectionWheel`
  (clear `self.OnOpenSelectionWheelPressed`)
  (clear `self.OnOpenSelectionWheelReleased`))

(event `self.UnbindConstruction`
  (bind _previewplacableactor (`MainPlayer.PreviewPlacableActor` (`self.MainPlayer`)))
  (`KismetSystemLibrary.K2_ClearAndInvalidateTimerHandle` (`self.PreviewObjectTimerHandle`))
  (`KismetSystemLibrary.K2_ClearAndInvalidateTimerHandle` (`self.CanBePlaceTimerHandle`))
  (clear `self.OnPlaceObject`)
  (`self.UnbindRotateObjects`)
  (`/Engine/EditorBlueprintResources/StandardMacros.IsValid` _previewplacableactor
    (:`Is Valid`
      (`PreviewPlacableActor.ResetActor` _previewplacableactor))))

(fn `BindClingMovement`
  (`self.UnbindMovement`)
  (`self.UnbindInteraction`)
  (clear `self.OnUseGlitchPressed`)
  (add `self.OnMoveForward` (`|CreateDelegate` (`self.MainPlayer`) :!event `ClingUp`))
  (add `self.OnMoveRight` (`|CreateDelegate` (`self.MainPlayer`) :!event `ClingRight`))
  (return))

(fn `BindRotateObjects`
  (`self.UnbindRotateObjects`)
  (add `self.OnRotateObjects` (`|CreateDelegate` :!event `Rotate Object`))
  (add `self.OnRotateObjectsLeft` (`|CreateDelegate` :!event `Rotate Object`))
  (add `self.OnRotateObjectsRight` (`|CreateDelegate` :!event `Rotate Object`))
  (return))

(fn `CloseWheel`
  (if (<= (`KismetSystemLibrary.K2_GetTimerElapsedTimeHandle` (`self.OpenWheelTimer`)) 0.05)
    (`self.SelectNewGameplayMode` "CPF_Normal")
    ;[1 0 0] Temp
    (bind _outactors (`GameplayStatics.GetAllActorsOfClass` "/Game/Blueprint/PlacableObjects/BP_ConstructionZone.BP_ConstructionZone_C"))
    (for _array_element _outactors
      (if (`|EnumEquality` (`ActivableComponent.GetState` (`ConstructionZone.GetActivableComp` _array_element)) "CPF_Activated")
        (`SceneComponent.SetVisibility` (`/Game/Blueprint/PlacableObjects/BP_ConstructionZone.VisibilityPlane` _array_element) false false))))
  (`KismetSystemLibrary.K2_ClearAndInvalidateTimerHandle` (`self.OpenWheelTimer`))
  (`Widget.RemoveFromParent` (`self.PlacableObjectWheel`))
  (`GameplayStatics.SetGlobalTimeDilation` 1.0)
  (`self.BindCamera`)
  (`WidgetBlueprintLibrary.SetInputMode_GameOnly` self)
  (set `self.bShowMouseCursor` false)
  (return))

(fn `DisplayWaveManagerUI`
  (`UserWidget.AddToViewport` (`self.WaveManagerUI`) 0)
  (`self.UnbindAll`)
  (add `self.OnPause` (`|CreateDelegate` :!event `RemoveWaveManagerUI`))
  (add `self.OnInteractPlayer` (`|CreateDelegate` :!event `RemoveWaveManagerUI`))
  (return))

(fn `GetCurrentPlacableObject`
  (returns (Class :type "PlacableActor Class Reference") (Data :type "PlacableActorData Object Reference"))
  (bind (_class _data) (`self.GetPlacableObject` (`self.CurrentPlacableObjectIndex`)))
  (return _class _data))

(fn `GetPlacableObject`
  (params (Index :type Integer))
  (returns (Class :type "PlacableActor Class Reference") (Data :type "PlacableActorData Object Reference"))
  (bind (_class _data) (break `PlacableActorCreation` (`|GetArrayItem` (`self.PlacableObjectList`) Index)))
  (return _class _data))

(fn `Open`
  (bind _returnvalue (`KismetSystemLibrary.K2_SetTimerDelegate` (`|CreateDelegate` :!event `OpenWheel`) 0.05 false 0.05))
  (set `self.OpenWheelTimer` _returnvalue)
  (return))

(fn `OpenWheel`
  (bind _placableobjectwheel (`self.PlacableObjectWheel`))
  (`UserWidget.AddToViewport` _placableobjectwheel 0)
  (`WidgetBlueprintLibrary.SetInputMode_GameAndUIEx` self _placableobjectwheel)
  (`self.UnbindCamera`)
  (set `self.bShowMouseCursor` true)
  (`GameplayStatics.SetGlobalTimeDilation` 0.2)
  (return))

(fn `RemoveConstructionUI`
  (`Widget.RemoveFromParent` (`self.PlacableObjectWheel`))
  (return))

(fn `RemoveWaveManagerUI`
  (`Widget.RemoveFromParent` (`self.WaveManagerUI`))
  (`self.SelectNewGameplayMode` (`self.GetGameplayMode`))
  (return))

(fn `Rotate Object`
  (params (AxisValue :type "Float (double-precision)"))
  (if (!= AxisValue 0.0)
    (switch `int` (`KismetMathLibrary.FTrunc` (`local.AxisValue`))
      (:`-1`
        (`/Game/Blueprint/Player/BP_MainPlayer.RotateActor` (`self.MainPlayer`) (struct :`Yaw` -90.0))
        (return))
      (:`1`
        (`/Game/Blueprint/Player/BP_MainPlayer.RotateActor` (`self.MainPlayer`) (struct :`Yaw` 90.0))
        (return)))))

(fn `ShowConstructionUI`
  (`/Game/Blueprint/Helpers/FunctionLibrary/BP_UsefullFunctions.SecurAddToViewport` (`self.PlacableObjectWheel`))
  (return))

(fn `UnbindRotateObjects`
  (clear `self.OnRotateObjects`)
  (clear `self.OnRotateObjectsLeft`)
  (clear `self.OnRotateObjectsRight`)
  (return))

(fn `UserConstructionScript`)