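; Player controller for the main menu that shows an intro widget, or goes straight to the title menu when the game mode options equal "?SkipIntro".
; On BeginPlay it creates the title widget, then either shows the intro and binds to OnInteractPlayer, which any key fires, or calls CreateMainMenuWidget.
; That function shows the cursor, clears the interact bindings, displays the title and loops the LS_MainMenu sequence.
; Pause input fires OnPause.
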(event `self.ReceiveBeginPlay`
  (bind _returnvalue (`|CreateWidget` "/Game/Blueprint/Menu/MainMenu/WBP_MainTitle.WBP_MainTitle_C"))
  (set `self.MainMenuWidget` _returnvalue)
  (if (`KismetStringLibrary.NotEqual_StrStr` (`GameModeBase.OptionsString` (`GameplayStatics.GetGameMode`)) "?SkipIntro")
    (bind _returnvalue_2 (`|CreateWidget` "/Game/Blueprint/Menu/MainMenu/WBP_Introduction.WBP_Introduction_C"))
    (bind _output_get (set `self.IntroWidget` _returnvalue_2))
    (`UserWidget.AddToViewport` _output_get 0)
    (add `self.OnInteractPlayer` (`|CreateDelegate` (`self.IntroWidget`) :!event `SkipAnim`))
    (else
      (`self.CreateMainMenuWidget`))))

(event `Key|AnyKey`
  (params (Key :type "Key Structure"))
  (:`Pressed`
    (`self.OnInteractPlayer`)))

(event `InputAction|Pause`
  (params (Key :type "Key Structure"))
  (:`Pressed`
    (`self.OnPause`)))

(fn `CreateMainMenuWidget`
  (bind _returnvalue (`GameplayStatics.GetPlayerController` 0))
  (set `PlayerController.bShowMouseCursor` true _returnvalue)
  (clear `self.OnInteractPlayer` (cast `/Game/Blueprint/Player/Controllers/BP_PC_MenuController` _returnvalue :!pure true))
  (`UserWidget.AddToViewport` (`self.MainMenuWidget`) 0)
  (bind (_outactor _returnvalue_2) (`LevelSequencePlayer.CreateLevelSequencePlayer` "/Game/Animation/LevelSequance/LS_MainMenu.LS_MainMenu"))
  (`MovieSceneSequencePlayer.PlayLooping` _returnvalue_2 -1)
  (return))

(fn `UserConstructionScript`)