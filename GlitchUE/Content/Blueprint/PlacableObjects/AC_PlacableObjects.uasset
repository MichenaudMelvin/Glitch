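; AC_PlacableObjects is an actor component that supports placeable objects with a placement check, a reset and a mesh swap.
; CanBePlaced runs a zero-length Visibility box trace just above the owner, with persistent debug drawing, and returns true when nothing is hit.
; ResetOBJ clears the box trace timer before calling ResetObject.
; SetOwnerStaticMesh casts the owner to BP_PlacableActorWithMesh and replaces its static mesh.
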(fn `Can be Placed`
  (bind _returnvalue (`KismetMathLibrary.MakeVector` (.x (`Actor.K2_GetActorLocation` (`self.GetOwner`))) (.y (`Actor.K2_GetActorLocation` (`self.GetOwner`))) (+ (.z (`Actor.K2_GetActorLocation` (`self.GetOwner`))) 30.0)))
  (bind (_outhit _returnvalue_2) (`KismetSystemLibrary.BoxTraceSingle` :`Start` _returnvalue :`End` _returnvalue :`HalfSize` (25.0 25.0 25.0) :`TraceChannel` "TraceTypeQuery1" :`DrawDebugType` "Persistent"))
  (set `self.CanBePlaced` (not _returnvalue_2))
  (return))

(fn `ResetOBJ`
  (`KismetSystemLibrary.K2_ClearAndInvalidateTimerHandle` (`self.BoxTraceTimerHandle`))
  (`self.ResetObject`)
  (return))

(fn `SetOwnerStaticMesh`
  (params (NewMesh :type "StaticMesh Object Reference"))
  (`StaticMeshComponent.SetStaticMesh` (`/Game/Blueprint/PlacableObjects/BP_PlacableActorWithMesh.StaticMesh` (cast `/Game/Blueprint/PlacableObjects/BP_PlacableActorWithMesh` (`self.GetOwner`) :!pure true)) NewMesh)
  (return))