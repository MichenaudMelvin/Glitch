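; Railgun turret, a placeable defense that fires a piercing beam at AI enemies, with a construction effect on spawn.
; Parent attack events drive the cycle: unfold the head if folded, aim, shoot, play the destruction animation, then cool down.
; Shoot box-traces from the crystal socket past the target, damaging each unique enemy until a static mesh or nine hits stop it.
; PopcornFX emitters receive position attributes to draw the beam and appearance effect.
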(event `self.ReceiveBeginPlay`
  (`parent.ReceiveBeginPlay`)
  (bind _returnvalue (`PopcornFXFunctions.SpawnEmitterAtLocation` "/Game/VFX/Particles/FX_Towers/FX_Sniper/Pk_Construct_Sniper.Pk_Construct_Sniper" "PopcornFX_DefaultScene" (0.0 0.0 0.0) (struct) false false))
  (set `self.AppearenceFX` _returnvalue)
  (`self.MakeAppear`)
  (`self.SetObjectMaterial` "/Game/VFX/Shaders/ConstructionNumeric/M_Construct_Inst.M_Construct_Inst"))

(event `self.EndAppearence`
  (`parent.EndAppearence`)
  (`self.SetObjectMaterial` "/Game/Meshs/Materials/M_Constent_MED_Mats.M_Constent_MED_Mats"))

(event `self.Attack`
  (bind _constructionanim (`self.ConstructionAnim`))
  (`parent.Attack`)
  (if (`self.IsDestruct`)
    (`SkeletalMeshComponent.PlayAnimation` (`self.TurretHead`) _constructionanim false)
    (set `self.IsDestruct` false)
    (bind _returnvalue (`AnimSequenceBase.GetPlayLength` _constructionanim))
    (`KismetSystemLibrary.Delay` _returnvalue))
  (`self.LookAtTarget`))

(event `self.EndRotate`
  (`parent.EndRotate`)
  (`/Engine/EditorBlueprintResources/StandardMacros.IsValid` (`self.CurrentTarget`)
    (:`Is Valid`
      (`SkeletalMeshComponent.PlayAnimation` (`self.TurretHead`) (`self.AttackAnimation`) false)
      (`self.Shoot`)
      (bind _returnvalue (`AnimSequenceBase.GetPlayLength` (`self.AttackAnimation`)))
      (`KismetSystemLibrary.Delay` _returnvalue)
      (`SkeletalMeshComponent.PlayAnimation` (`self.TurretHead`) (`self.DestructionAnim`) false)
      (set `self.IsDestruct` true)
      (`KismetSystemLibrary.Delay` (/ (`self.AttackRate`) 2.0)))
    (:`Is Not Valid`
      _))
  (`self.EndAttack`))

(event `self.FinishAttacking`
  (`parent.FinishAttacking`)
  (if (`self.IsDestruct`)
    (`SkeletalMeshComponent.PlayAnimation` (`self.TurretHead`) (`self.ConstructionAnim`) false)
    (set `self.IsDestruct` false)))

(event `BreakRail`
  (goto _label :!via `Break`))

(event `self.Shoot`
  (bind _attackfx (`self.AttackFX`))
  (bind _attackfx_2 (`self.AttackFX`))
  (bind _returnvalue (+ (`self.K2_GetActorLocation` (`self.CurrentTarget`)) (* (`SceneComponent.GetForwardVector` (`self.TurretHead`)) (`self.AttackRange`))))
  (`parent.Shoot`)
  (`|SetAttribute` _attackfx (`PopcornFXAttributeFunctions.FindAttributeIndex` _attackfx "TargetPosition") true "Vector" _returnvalue)
  (`|SetAttribute` _attackfx_2 (`PopcornFXAttributeFunctions.FindAttributeIndex` _attackfx_2 "StartPosition") true "Vector" (`self.GetShootStartLocation`))
  (`PopcornFXEmitterComponent.StartEmitter` (`self.AttackFX`))
  (bind _outhits (`KismetSystemLibrary.BoxTraceMulti` (`self.GetShootStartLocation`) _returnvalue (20.0 20.0 20.0) (struct) "TraceTypeQuery4"))
  (for _array_element _outhits :!label _label
    (bind (_bblockinghit _binitialoverlap _time _distance _location _impactpoint _normal _impactnormal _physmat _hitactor _hitcomponent) (`GameplayStatics.BreakHitResult` _array_element))
    (if (`/Game/Blueprint/Helpers/FunctionLibrary/BP_UsefullFunctions.CheckTargetClass` _hitcomponent "/Script/Engine.StaticMeshComponent")
      (`self.BreakRail`)
      (elif (not (`BlueprintSetLibrary.Set_Contains` (`self.HittedAIList`) _hitactor))
        (bind (_returnvalue_2 _returnobject) (`/Game/Blueprint/Helpers/FunctionLibrary/BP_UsefullFunctions.CheckParentClass` _hitactor "/Script/GlitchUE.MainAICharacter"))
        (if _returnvalue_2
          (bind _asmain_aicharacter (cast `MainAICharacter` _returnobject :!pure true))
          (`BlueprintSetLibrary.Set_Add` (`self.HittedAIList`) _asmain_aicharacter)
          (`HealthComponent.TakeDamages` (`MainAICharacter.HealthComp` _asmain_aicharacter) (`self.Damages`))
          (if (== (`BlueprintSetLibrary.Set_Length` (`self.HittedAIList`)) 9)
            (`self.BreakRail`))))))
  (`BlueprintSetLibrary.Set_Clear` (`self.HittedAIList`)))

(fn `GetShootStartLocation`
  (returns (ReturnValue :type "Vector Structure"))
  (return (`SceneComponent.GetSocketLocation` (`self.TurretHead`) "Railgun_Crystal")))

(fn `MakeAppear`
  (bind _appearencefx (`self.AppearenceFX`))
  (bind _appearencefx_2 (`self.AppearenceFX`))
  (`|SetAttribute` _appearencefx (`PopcornFXAttributeFunctions.FindAttributeIndex` _appearencefx "PositionInWorld") true "Vector" (`self.K2_GetActorLocation`))
  (`|SetAttribute` _appearencefx_2 (`PopcornFXAttributeFunctions.FindAttributeIndex` _appearencefx_2 "Orientation") "Rotator" (`self.K2_GetActorRotation`))
  (`PopcornFXEmitterComponent.StartEmitter` (`self.AppearenceFX`))
  (return))

(fn `UserConstructionScript`)