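; Placeable turret that automatically attacks AI characters inside its box-shaped range.
; Overlap events maintain the target list, and the first entry starts a self-repeating, delayed Attack loop that runs until the list empties.
; Each attack turns the pillar's yaw via timeline and instantly damages an AC_DestructibleObject, using separate random picks for aim and damage.
; SetData and SetMesh overrides apply damage, delay, range and meshes from data objects.
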(event `Attack`
  (bind _outitem (`KismetArrayLibrary.Array_Random` (`self.AIList`)))
  (if (> (`KismetArrayLibrary.Array_Length` (`self.AIList`)) 0)
    (`self.LookAtTarget` _outitem)
    (`/Game/Blueprint/DestructibleObjects/AC_DestructibleObject.TakeDamages` (`self.GetComponentByClass` _outitem "/Game/Blueprint/DestructibleObjects/AC_DestructibleObject.AC_DestructibleObject_C") (`self.Damages`))
    (`KismetSystemLibrary.Delay` (`self.DelayBetweenEachAttack`))
    (`self.Attack`)))

(event `self.TurretRadius.OnComponentBeginOverlap`
  (params (OverlappedComponent :type "PrimitiveComponent Object Reference") (OtherActor :type "Actor Object Reference") (OtherComp :type "PrimitiveComponent Object Reference") (OtherBodyIndex :type Integer) (bFromSweep :type Boolean) (SweepResult :type "HitResult Structure (by ref)"))
  (bind (_returnvalue _returnobject) (`/Game/Blueprint/Helpers/FunctionLibrary/BP_UsefullFunctions.CheckParentClass` OtherActor "/Game/Blueprint/AI/BP_MainAICharacter.BP_MainAICharacter_C"))
  (if _returnvalue
    (`KismetArrayLibrary.Array_Add` (`self.AIList`) (cast `/Game/Blueprint/AI/BP_MainAICharacter` _returnobject :!pure true))
    (if (== (`KismetArrayLibrary.Array_Length` (`self.AIList`)) 1)
      (`self.Attack`))))

(event `self.TurretRadius.OnComponentEndOverlap`
  (params (OverlappedComponent :type "PrimitiveComponent Object Reference") (OtherActor :type "Actor Object Reference") (OtherComp :type "PrimitiveComponent Object Reference") (OtherBodyIndex :type Integer))
  (bind (_returnvalue _returnobject) (`/Game/Blueprint/Helpers/FunctionLibrary/BP_UsefullFunctions.CheckParentClass` OtherActor "/Game/Blueprint/AI/BP_MainAICharacter.BP_MainAICharacter_C"))
  (if _returnvalue
    (`KismetArrayLibrary.Array_RemoveItem` (`self.AIList`) (cast `/Game/Blueprint/AI/BP_MainAICharacter` _returnobject :!pure true))))

(event `LookAtTarget`
  (params (Target :type "Actor Object Reference"))
  (set `self.CurrentZRotation` (.yaw (`SceneComponent.K2_GetComponentRotation` (`self.TurretPillar`))))
  (bind (_direction _alpha) (`Timeline|RotateTimeline` :!via `PlayFromStart`)
    (:`Update`
      (`SceneComponent.K2_SetWorldRotation` (`self.TurretPillar`) (`KismetMathLibrary.MakeRotator` 0.0 0.0 (`KismetMathLibrary.Lerp` (`self.CurrentZRotation`) (.yaw (`KismetMathLibrary.FindLookAtRotation` (`self.K2_GetActorLocation`) (`self.K2_GetActorLocation` Target))) _alpha)) false false))))

(fn `SetData`
  (params (CurrentData :type "/Game/Blueprint/PlacableObjects/BP_PlacableActorData Object Reference"))
  (bind _asbp_turret_data (cast `/Game/Blueprint/PlacableObjects/Turrets/BP_TurretData` CurrentData :!pure true))
  (bind _turretradius (`/Game/Blueprint/PlacableObjects/Turrets/BP_TurretData.TurretRadius` _asbp_turret_data))
  (`parent.SetData` CurrentData)
  (set `self.Damages` (`/Game/Blueprint/PlacableObjects/Turrets/BP_TurretData.Damages` _asbp_turret_data))
  (set `self.DelayBetweenEachAttack` (`/Game/Blueprint/PlacableObjects/Turrets/BP_TurretData.DelayBetweenEachAttack` _asbp_turret_data))
  (`BoxComponent.SetBoxExtent` (`self.TurretRadius`) (`KismetMathLibrary.MakeVector` _turretradius _turretradius 100.0) false)
  (return))

(fn `SetMesh`
  (params (Data :type "/Game/Blueprint/PlacableObjects/BP_PlacableActorData Object Reference"))
  (bind _staticmeshlist (`/Game/Blueprint/PlacableObjects/BP_PlacableActorDataWithMesh.StaticMeshList` (cast `/Game/Blueprint/PlacableObjects/BP_PlacableActorDataWithMesh` Data :!pure true)))
  (`parent.SetMesh` Data)
  (`StaticMeshComponent.SetStaticMesh` (`self.TurretPillar`) (`|GetArrayItem` _staticmeshlist 1))
  (`StaticMeshComponent.SetStaticMesh` (`self.TurretHead`) (`|GetArrayItem` _staticmeshlist 2))
  (return))

(fn `UserConstructionScript`
  (`parent.UserConstructionScript`))