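; Crossbow turret, a child of a base turret, that appears with a construction effect and material, then attacks AI characters in its radius.
; Overlaps start and stop a looping timer; Attack aims at the target, and EndRotate plays the shot.
; Arrows are purely visual PopcornFX emitters driven by attributes: damage hits the target's health component directly after the animation's length.
; After the fire-rate delay, it retargets the first listed AI and repeats.
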(event `self.ReceiveBeginPlay`
  (bind _shootfx (`self.ShootFX`))
  (bind _shootfx_2 (`self.ShootFX`))
  (`parent.ReceiveBeginPlay`)
  (bind _returnvalue (`PopcornFXFunctions.SpawnEmitterAtLocation` "/Game/VFX/Particles/FX_Towers/FX_Crossbow/Pk_ArrowShotStraight.Pk_ArrowShotStraight" "PopcornFX_DefaultScene" (0.0 0.0 0.0) (struct) false false))
  (bind _output_get (set `self.ShootFX` _returnvalue))
  (`|SetAttribute` _output_get (`PopcornFXAttributeFunctions.FindAttributeIndex` (`self.ShootFX`) "Turret") true "Vector" (`SceneComponent.K2_GetComponentLocation` (`self.TurretHead`)))
  (`|SetAttribute` _shootfx_2 (`PopcornFXAttributeFunctions.FindAttributeIndex` _shootfx_2 "LifeTimeArrow") true "Float" 0.7)
  (`|SetAttribute` _shootfx (`PopcornFXAttributeFunctions.FindAttributeIndex` _shootfx "DistanceValidator") true "Float" 0.7)
  (bind _returnvalue_2 (`PopcornFXFunctions.SpawnEmitterAtLocation` "/Game/VFX/Particles/FX_Towers/FX_Crossbow/Pk_Construct_Crossbow.Pk_Construct_Crossbow" "PopcornFX_DefaultScene" (0.0 0.0 0.0) (struct) false false))
  (set `self.TurretAppearenceFX` _returnvalue_2)
  (`self.MakeAppear`)
  (`self.SetObjectMaterial` "/Game/VFX/Shaders/ConstructionNumeric/M_Construct_Inst.M_Construct_Inst"))

(event `self.EndAppearence`
  (`parent.EndAppearence`)
  (`self.SetObjectMaterial` "/Game/Meshs/Materials/M_Constent_MED_Mats.M_Constent_MED_Mats"))

(event `self.Attack`
  (`parent.Attack`)
  (`self.LookAtTarget`))

(event `self.EndRotate`
  (`parent.EndRotate`)
  (`SkeletalMeshComponent.PlayAnimation` (`self.TurretHead`) (`self.ShootAnim`) false)
  (`self.Shoot`)
  (bind _returnvalue (`AnimSequenceBase.GetPlayLength` (`self.ShootAnim`)))
  (`KismetSystemLibrary.Delay` _returnvalue)
  (`HealthComponent.TakeDamages` (`MainAICharacter.HealthComp` (cast `/Game/Blueprint/AI/BP_MainAICharacter` (`self.CurrentTarget`) :!pure true)) (`self.Damages`))
  (`KismetSystemLibrary.Delay` (`self.FireRate`))
  (if (`self.DoesAIListContainSomething`)
    (set `self.CurrentTarget` (`self.GetFirstAI`))
    (`self.Attack`)))

(event `self.TurretRadius.OnComponentBeginOverlap`
  (params (OverlappedComponent :type "PrimitiveComponent Object Reference") (OtherActor :type "Actor Object Reference") (OtherComp :type "PrimitiveComponent Object Reference") (OtherBodyIndex :type Integer) (bFromSweep :type Boolean) (SweepResult :type "HitResult Structure (by ref)"))
  (`self.BeginOverlap` OtherActor))

(event `self.BeginOverlap`
  (params (OverlappedActor :type "Actor Object Reference"))
  (`parent.BeginOverlap` OverlappedActor)
  (if (== (`BlueprintSetLibrary.Set_Length` (`self.AIList`)) 1)
    (bind _returnvalue (`KismetSystemLibrary.K2_SetTimerDelegate` (`|CreateDelegate` :!event `CanAttack`) 0.1 true))
    (set `self.CanAttackTimer` _returnvalue)))

(event `self.TurretRadius.OnComponentEndOverlap`
  (params (OverlappedComponent :type "PrimitiveComponent Object Reference") (OtherActor :type "Actor Object Reference") (OtherComp :type "PrimitiveComponent Object Reference") (OtherBodyIndex :type Integer))
  (`self.EndOverlap` OtherActor))

(event `self.EndOverlap`
  (params (OverlappedActor :type "Actor Object Reference"))
  (`parent.EndOverlap` OverlappedActor)
  (if (== (`BlueprintSetLibrary.Set_Length` (`self.AIList`)) 0)
    (`KismetSystemLibrary.K2_ClearAndInvalidateTimerHandle` (`self.CanAttackTimer`))))

(fn `MakeAppear`
  (bind _turretappearencefx (`self.TurretAppearenceFX`))
  (bind _turretappearencefx_2 (`self.TurretAppearenceFX`))
  (`|SetAttribute` _turretappearencefx (`PopcornFXAttributeFunctions.FindAttributeIndex` _turretappearencefx "PositionInWorld") true "Vector" (`self.K2_GetActorLocation`))
  (`|SetAttribute` _turretappearencefx_2 (`PopcornFXAttributeFunctions.FindAttributeIndex` _turretappearencefx_2 "Orientation") "Rotator" (`self.K2_GetActorRotation`))
  (`PopcornFXEmitterComponent.StartEmitter` (`self.TurretAppearenceFX`))
  (return))

(fn `Shoot`
  (bind _shootfx (`self.ShootFX`))
  (`|SetAttribute` _shootfx (`PopcornFXAttributeFunctions.FindAttributeIndex` _shootfx "Target") true "Vector" (`self.K2_GetActorLocation` (`self.CurrentTarget`)))
  (`PopcornFXEmitterComponent.StartEmitter` (`self.ShootFX`))
  (return))

(fn `UserConstructionScript`)