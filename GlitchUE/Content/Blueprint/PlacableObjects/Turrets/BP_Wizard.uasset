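; Wizard turret, a placeable that damages AI characters with a magical shot particle effect, extending a parent turret's attack.
; On BeginPlay it spawns a reusable, inactive shot emitter and binds its emission-stop event.
; Attack starts the cast effect, waits half the attack rate, plays the shot at the target's XY just above turret height, then waits again before ending.
; Damage is timed to the particle emission stopping, hitting whichever target is then current.
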(event `self.ReceiveBeginPlay`
  (`parent.ReceiveBeginPlay`)
  (bind _returnvalue (`PopcornFXFunctions.SpawnEmitterAtLocation` "/Game/VFX/Particles/FX_Towers/FX_Magical/Pk_MagicalShot.Pk_MagicalShot" "PopcornFX_DefaultScene" (0.0 0.0 0.0) (struct) false false))
  (bind _output_get (set `self.Shot` _returnvalue))
  (add `PopcornFXEmitterComponent.OnEmissionStops` _output_get (`|CreateDelegate` :!event `OnShotStop`)))

(event `self.Attack`
  (bind _shot (`self.Shot`))
  (`parent.Attack`)
  (`PopcornFXEmitterComponent.StartEmitter` (`self.AttackFX`))
  (`KismetSystemLibrary.Delay` (/ (`self.AttackRate`) 2.0))
  (`SceneComponent.K2_SetRelativeLocation` _shot (`KismetMathLibrary.MakeVector` (.x (`self.K2_GetActorLocation` (`self.CurrentTarget`))) (.y (`self.K2_GetActorLocation` (`self.CurrentTarget`))) (+ (.z (`self.K2_GetActorLocation`)) 10.0)) false false)
  (`PopcornFXEmitterComponent.StartEmitter` _shot)
  (`KismetSystemLibrary.Delay` (/ (`self.AttackRate`) 2.0))
  (`self.EndAttack`))

(event `OnShotStop`
  (params (EmitterComponent :type "PopcornFXEmitterComponent Object Reference") (Location :type "Vector Structure") (Rotation :type "Vector Structure"))
  (bind _currenttarget (`self.CurrentTarget`))
  (`/Engine/EditorBlueprintResources/StandardMacros.IsValid` _currenttarget
    (:`Is Valid`
      (`HealthComponent.TakeDamages` (`MainAICharacter.HealthComp` (cast `MainAICharacter` _currenttarget :!pure true)) (`self.Damages`)))))

(fn `UserConstructionScript`)