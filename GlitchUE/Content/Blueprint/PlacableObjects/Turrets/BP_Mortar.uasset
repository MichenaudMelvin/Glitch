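; BP_Mortar is a placeable turret that deals area damage around its current target.
; Attack replays a muzzle effect pre-spawned at BeginPlay, waits the attack rate, calls Shoot, then waits again before ending.
; Shoot spawns an explosion at the target's XY near the mortar's height and box-traces around the target, damaging each MainAICharacter once via a temporary hit list.
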(event `self.ReceiveBeginPlay`
  (`parent.ReceiveBeginPlay`)
  (bind _returnvalue (`PopcornFXFunctions.SpawnEmitterAtLocation` "/Game/VFX/Particles/FX_Towers/FX_Mortar/Pk_MortarShot.Pk_MortarShot" "PopcornFX_DefaultScene" (`UsefullFunctions.AddToVector` (`self.K2_GetActorLocation`) 0.0 0.0 10.0) (struct) false false))
  (set `self.ShotFX` _returnvalue))

(event `self.Attack`
  (`parent.Attack`)
  (`PopcornFXEmitterComponent.StartEmitter` (`self.ShotFX`))
  (`KismetSystemLibrary.Delay` (`self.AttackRate`))
  (`self.Shoot`)
  (`KismetSystemLibrary.Delay` (`self.AttackRate`))
  (`self.EndAttack`))

(event `self.Shoot`
  (bind _currenttarget (`self.CurrentTarget`))
  (bind _returnvalue (`self.K2_GetActorLocation` _currenttarget))
  (`parent.Shoot`)
  (`/Engine/EditorBlueprintResources/StandardMacros.IsValid` _currenttarget
    (:`Is Valid`
      (bind _outhits (`KismetSystemLibrary.BoxTraceMulti` _returnvalue _returnvalue (300.0 300.0 200.0) (struct) "TraceTypeQuery4"))
      (bind _returnvalue_2 (`PopcornFXFunctions.SpawnEmitterAtLocation` "/Game/VFX/Particles/FX_Towers/FX_Mortar/Pk_MortarExplosion.Pk_MortarExplosion" "PopcornFX_DefaultScene" (`KismetMathLibrary.MakeVector` (.x (`self.K2_GetActorLocation` (`self.CurrentTarget`))) (.y (`self.K2_GetActorLocation` (`self.CurrentTarget`))) (+ (.z (`self.K2_GetActorLocation`)) 10.0)) (struct) false false))
      (`PopcornFXEmitterComponent.StartEmitter` _returnvalue_2)
      (for _array_element _outhits
        (bind (_bblockinghit _binitialoverlap _time _distance _location _impactpoint _normal _impactnormal _physmat _hitactor) (`GameplayStatics.BreakHitResult` _array_element))
        (if (not (`BlueprintSetLibrary.Set_Contains` (`self.HittedAIList`) _hitactor))
          (bind (_returnvalue_3 _returnobject) (`/Game/Blueprint/Helpers/FunctionLibrary/BP_UsefullFunctions.CheckParentClass` _hitactor "/Script/GlitchUE.MainAICharacter"))
          (if _returnvalue_3
            (bind _asmain_aicharacter (cast `MainAICharacter` _returnobject :!pure true))
            (`BlueprintSetLibrary.Set_Add` (`self.HittedAIList`) _asmain_aicharacter)
            (`HealthComponent.TakeDamages` (`MainAICharacter.HealthComp` _asmain_aicharacter) (`self.Damages`)))))
      (`BlueprintSetLibrary.Set_Clear` (`self.HittedAIList`)))))

(fn `UserConstructionScript`)