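; BP_ConstructionZone is a placeable slot actor that shows a particle effect while it is active and available for a unit.
; At BeginPlay it spawns a dormant, persistent construction emitter just above the bottom of its collision box.
; Activation starts the effect, while deactivation or an occupying unit stops it.
; Freeing the slot restarts the effect if the zone is still active, with slot logic inherited from the parent.
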(event `self.ReceiveBeginPlay`
  (`parent.ReceiveBeginPlay`)
  (bind _returnvalue (`PopcornFXFunctions.SpawnEmitterAtLocation` "/Game/VFX/Particles/FX_Environment/Pk_ConstructionZone.Pk_ConstructionZone" "PopcornFX_DefaultScene" (`KismetMathLibrary.MakeVector` (.x (`self.K2_GetActorLocation`)) (.y (`self.K2_GetActorLocation`)) (+ (- (.z (`self.K2_GetActorLocation`)) (.z (`BoxComponent.BoxExtent` (cast `BoxComponent` (`self.CollisionComponent`) :!pure true)))) 5.0)) (struct) false false))
  (set `self.ConstructionFX` _returnvalue))

(event `self.ActivableComp.OnActivated`
  (`PopcornFXEmitterComponent.StartEmitter` (`self.ConstructionFX`)))

(event `self.OccupiedSlot`
  (params (NewUnit :type "PlacableActor Object Reference"))
  (`parent.OccupiedSlot` NewUnit)
  (`PopcornFXEmitterComponent.StopEmitter` (`self.ConstructionFX`) false))

(event `self.ActivableComp.OnDesactivated`
  (`PopcornFXEmitterComponent.StopEmitter` (`self.ConstructionFX`) false))

(event `self.UnoccupiedSlot`
  (`parent.UnoccupiedSlot`)
  (if (`ActivableComponent.IsActivated` (`self.ActivableComp`))
    (`PopcornFXEmitterComponent.StartEmitter` (`self.ConstructionFX`))))

(fn `UserConstructionScript`)