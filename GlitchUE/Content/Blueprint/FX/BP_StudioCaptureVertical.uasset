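; Studio rig that renders a scaled-down proxy of the level's BP_TransitionSphereVertical actors through a SceneCapture2D, apparently for a vertical transition effect.
; Shortly after BeginPlay, it builds a map pairing each sphere actor with a spawned black sphere mesh.
; UpdateRender captures the scene, then repositions proxies at 1/100 scale on the Y-Z plane with Z flipped and offset, so captures show the previous update's transforms.
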(event `self.ReceiveBeginPlay`
  (`KismetSystemLibrary.Delay` 0.2)
  (`self.Updating`))

(event `UpdateRender`
  (`SceneCaptureComponent2D.CaptureScene` (`self.SceneCaptureComponent2D`))
  (bind _keys (`BlueprintMapLibrary.Map_Keys` (`self.SceneProbes`)))
  (for _array_element _keys
    (`self.TransformEachComponent` _array_element)))

(fn `TransformEachComponent`
  (params (Key :type "/Game/Blueprint/FX/BP_TransitionSphereVertical Object Reference (by ref)"))
  (bind _output_get (set `self.ComponentToTransform` (`BlueprintMapLibrary.Map_Find` (`self.SceneProbes`) Key)))
  (`SceneComponent.K2_SetRelativeTransform` _output_get (`KismetMathLibrary.MakeTransform` (`KismetMathLibrary.MakeVector` 0.0 (.y (/ (.location (`self.GetTransform` (`local.Key`))) 100.0)) (+ (* -1 (.z (/ (.location (`self.GetTransform` (`local.Key`))) 100.0))) -1.8)) (struct) (/ (.scale (`self.GetTransform` (`local.Key`))) 100.0)) false false))

(fn `Updating`
  (locals (ActorsOutput :type "Array of /Game/Blueprint/FX/BP_TransitionSphereVertical Object Reference"))
  (bind _sceneprobes (`self.SceneProbes`))
  (bind _outactors (`GameplayStatics.GetAllActorsOfClass` "/Game/Blueprint/FX/BP_TransitionSphereVertical.BP_TransitionSphereVertical_C"))
  (set `local.ActorsOutput` _outactors)
  (if (not (== (`KismetArrayLibrary.Array_Length` _outactors) (`BlueprintMapLibrary.Map_Length` (`self.SceneProbes`))))
    (bind _values (`BlueprintMapLibrary.Map_Values` _sceneprobes))
    (for _array_element _values
      (`ActorComponent.K2_DestroyComponent` _array_element))
    (`BlueprintMapLibrary.Map_Clear` _sceneprobes)
    (for _array_element_2 (`local.ActorsOutput`)
      (bind _returnvalue (`AddComponent|NODE_AddStaticMeshComponent-2`))
      (`StaticMeshComponent.SetStaticMesh` _returnvalue "/Game/StarterContent/Shapes/Shape_Sphere.Shape_Sphere")
      (`PrimitiveComponent.SetMaterial` _returnvalue 0 "/Game/VFX/Shaders/RenderTargetDissolve/MI_Black.MI_Black")
      (`BlueprintMapLibrary.Map_Add` (`self.SceneProbes`) _array_element_2 _returnvalue))))

(fn `UserConstructionScript`)