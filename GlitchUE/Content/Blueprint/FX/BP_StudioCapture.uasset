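; BP_StudioCapture mirrors BP_TransitionSphere actors as black sphere meshes in a miniature top-down layout beside a SceneCaptureComponent2D.
; Updating rebuilds the actor-to-mesh map when the sphere count changes, then enables per-tick updates.
; Each tick scales world positions and sizes down by 160, rotates XY a quarter turn and flattens Z for the relative transforms.
; The manual CaptureScene call is disconnected.
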(event `UpdateRender`
  (bind _keys (`BlueprintMapLibrary.Map_Keys` (`self.SceneProbes`)))
  (for _array_element _keys
    (`self.TransformEachComponent` _array_element)))

(event `self.ReceiveTick`
  (params (DeltaSeconds :type "Float (single-precision)"))
  (if (`self.ShouldUpdate`)
    (`self.UpdateRender`)))

(fn `TransformEachComponent`
  (params (Key :type "/Game/Blueprint/FX/BP_TransitionSphere Object Reference (by ref)"))
  (bind _output_get (set `self.ComponentToTransform` (`BlueprintMapLibrary.Map_Find` (`self.SceneProbes`) Key)))
  (`SceneComponent.K2_SetRelativeTransform` _output_get (`KismetMathLibrary.MakeTransform` (`KismetMathLibrary.MakeVector` (* -1 (.y (/ (.location (`self.GetTransform` (`local.Key`))) 160.0))) (.x (/ (.location (`self.GetTransform` (`local.Key`))) 160.0))) (struct) (/ (.scale (`self.GetTransform` (`local.Key`))) 160.0)) false false))

(fn `Updating`
  (locals (ActorsOutput :type "Array of /Game/Blueprint/FX/BP_TransitionSphere Object Reference"))
  (bind _sceneprobes (`self.SceneProbes`))
  (`|ExecutionSequence`
    (:`then_0`
      (bind _outactors (`GameplayStatics.GetAllActorsOfClass` "/Game/Blueprint/FX/BP_TransitionSphere.BP_TransitionSphere_C"))
      (set `local.ActorsOutput` _outactors)
      (if (not (== (`KismetArrayLibrary.Array_Length` _outactors) (`BlueprintMapLibrary.Map_Length` (`self.SceneProbes`))))
        (bind _values (`BlueprintMapLibrary.Map_Values` _sceneprobes))
        (for _array_element _values
          (`ActorComponent.K2_DestroyComponent` _array_element))
        (`BlueprintMapLibrary.Map_Clear` _sceneprobes)
        (for _array_element_2 (`local.ActorsOutput`)
          (bind _returnvalue (`AddComponent|NODE_AddStaticMeshComponent-2`))
          (`StaticMeshComponent.SetStaticMesh` _returnvalue "/Game/StarterContent/Shapes/Shape_Sphere.Shape_Sphere")
          (`PrimitiveComponent.SetMaterial` _returnvalue 0 "/Game/VFX/Shaders/RenderTargetDissolve/MI_Black.MI_Black")
          (`BlueprintMapLibrary.Map_Add` (`self.SceneProbes`) _array_element_2 _returnvalue))))
    (:`then_1`
      (set `self.ShouldUpdate` true))))

(fn `UserConstructionScript`)