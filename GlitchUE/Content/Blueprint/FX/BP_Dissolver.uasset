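; BP_Dissolver drives a radius-based world dissolve effect, with editor events that snap the environment between MED (max radius) and TECH (zero radius).
; It pushes its position, scale, radius and look settings into the MPC_Dissolver Material Parameter Collection on construction and BeginPlay, then resets the radius to zero.
; DissolveTo runs a timeline, rate-scaled by FXDuration, that lerps the radius, updating both the material parameter and DissolveCollider sphere.
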(event `self.ReceiveBeginPlay`
  (`self.UpdateShaderFX`)
  (set `self.Radius` 0.0)
  (`self.UpdateRadius`))

(event `UpdateRadius`
  (bind _radius (`self.Radius`))
  (`KismetMaterialLibrary.SetScalarParameterValue` "/Game/VFX/Shaders/Dissolver/MPC_Dissolver.MPC_Dissolver" "Radius Dissolve" _radius)
  (`SphereComponent.SetSphereRadius` (`self.Dissolve Collider`) _radius true))

(event `UpdateShaderFX`
  (bind _root (`self.Root`))
  (`KismetMaterialLibrary.SetVectorParameterValue` "/Game/VFX/Shaders/Dissolver/MPC_Dissolver.MPC_Dissolver" "Position 1" (`KismetMathLibrary.Conv_VectorToLinearColor` (`SceneComponent.K2_GetComponentLocation` _root)))
  (`KismetMaterialLibrary.SetVectorParameterValue` "/Game/VFX/Shaders/Dissolver/MPC_Dissolver.MPC_Dissolver" "Bounds" (`KismetMathLibrary.Conv_VectorToLinearColor` (`SceneComponent.K2_GetComponentScale` _root)))
  (`self.UpdateRadius`)
  (`KismetMaterialLibrary.SetVectorParameterValue` "/Game/VFX/Shaders/Dissolver/MPC_Dissolver.MPC_Dissolver" "Emissive" (`self.Emissive`))
  (`KismetMaterialLibrary.SetScalarParameterValue` "/Game/VFX/Shaders/Dissolver/MPC_Dissolver.MPC_Dissolver" "SecondTilling" (`self.SecondTilling`))
  (`KismetMaterialLibrary.SetScalarParameterValue` "/Game/VFX/Shaders/Dissolver/MPC_Dissolver.MPC_Dissolver" "Radus Scale" (`self.Radius Scale`))
  (`KismetMaterialLibrary.SetScalarParameterValue` "/Game/VFX/Shaders/Dissolver/MPC_Dissolver.MPC_Dissolver" "Power" (`self.Power`))
  (`KismetMaterialLibrary.SetScalarParameterValue` "/Game/VFX/Shaders/Dissolver/MPC_Dissolver.MPC_Dissolver" "Tex Rez" (`self.Tex Rez`))
  (`TimelineComponent.SetPlayRate` (`self.DissolveTimeline`) (/ 1.0 (`self.FXDuration`))))

(event `PlayFX`
  (set `self.CurrentRadiusValue` (`self.Radius`))
  (bind (_direction _value) (`Timeline|DissolveTimeline` :!via `PlayFromStart`)
    (:`Update`
      (set `self.Radius` (`KismetMathLibrary.Lerp` (`self.CurrentRadiusValue`) (`self.TargetRadiusValue`) _value))
      (`self.UpdateRadius`))))

(event `SetEnvironementToMED`
  ;[0.5 0.5 1] Editor
  (set `self.Radius` (`self.MaxRadius`))
  (`self.UpdateRadius`))

(event `SetEnvironnementToTECH`
  ;[0.5 0.5 1] Editor
  (set `self.Radius` 0.0)
  (`self.UpdateRadius`))

(fn `DissolveTo`
  (params (TargetRadius :type "Float (double-precision)"))
  (set `self.TargetRadiusValue` TargetRadius)
  (`self.PlayFX`)
  (return))

(fn `SetNewRadius`
  (params (Radus :type "Float (double-precision)"))
  (set `self.Radius` Radus))

(fn `UserConstructionScript`
  (`self.UpdateShaderFX`))