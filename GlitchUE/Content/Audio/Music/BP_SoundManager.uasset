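; BP_SoundManager is a music manager that drives parameters on an FMOD audio component from the game's state.
; Tick, gated by a 0.2-second Delay, checks whether the GlitchUEGameMode level state is Alerted and plays the Infiltration timeline.
; That timeline's volume track feeds the "Stealth" parameter, with no reverse path when the alert ends.
; A separate GlitchZone event passes its value straight to the "Glitch_Zone" parameter.
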(event `self.ReceiveTick`
  (params (DeltaSeconds :type "Float (single-precision)"))
  (`KismetSystemLibrary.Delay` 0.2)
  (if (`|EnumEquality` (`GlitchUEGameMode.GetLevelState` (cast `GlitchUEGameMode` (`GameplayStatics.GetGameMode`) :!pure true)) "Alerted")
    (bind (_direction _volume_infiltration) (`Timeline|Infiltration`)
      (:`Update`
        (`FMODAudioComponent.SetParameter` (`self.FMODAudio`) "Stealth" _volume_infiltration)))))

(event `GlitchZone`
  (params (Value :type "Float (double-precision)"))
  (`FMODAudioComponent.SetParameter` (`self.FMODAudio`) "Glitch_Zone" Value))

(fn `UserConstructionScript`)